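; Blueprint function library that runs quests for TikiTandems, tied to the training grounds controller and its UI.
; DT_Quests supplies definitions, while the game instance's StQuests array holds runtime state, indexed by the numeric quest ID minus one.
; Setting a quest starts its step count at 1, updates explanation and HUD widgets, then calls ExplanationPause.
; Progressing increments the count and HUD, marking completion when it equals the table's step total.
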(fn Equal(stQuest)
  (params (Struct1 :type ST%20Quest%20Structure) (Struct2 :type ST%20Quest%20Structure))
  (return (Utilities|String|Contains (Utilities|String|ToString(Text) (.QuestName (Utilities|Struct|BreakST_Quest Struct1))) (Utilities|String|ToString(Text) (.QuestName (Utilities|Struct|BreakST_Quest Struct2))))))

(fn TexttoInt
  (params (text :type Text))
  (return (Math|Conversions|ToInteger(Byte) (Utilities|String|ToString(Text) text))))

(fn NametoInt
  (params (name :type Name))
  (return (Math|Conversions|ToInteger(Byte) (Utilities|String|ToString(Name) name))))

(fn SetCurrentQuest
  (params (QuestID :type Name))
  (bind _quest (CallFunction|GetAnyQuestbyID QuestID))
  (bind _asgi_tiki_tandems (Utilities|Casting|CastToGI_TikiTandems (Game|GetGameInstance)))
  (Utilities|Array|SetArrayElem (Variables|/Game/Core/Blueprints/GameRules/GI_TikiTandems.GI_TikiTandems_C|GetstQuests _asgi_tiki_tandems) (- (CallFunction|NametoInt QuestID) 1) (Utilities|Struct|MakeST_Quest (.questname _quest) (.questdescription _quest) 1 false) true)
  (CallFunction|UpdateWidget QuestID)
  (bind _asbpc_training_grounds (Utilities|Casting|CastToBPC_TrainingGrounds (Game|GetPlayerController 0)))
  (Default|ExplanationPause _asbpc_training_grounds))

(fn GetAnyQuestbyID
  (params (Row :type Name))
  (bind _returnvalue (Utilities|GetDataTableRow "/Game/Core/Data/CharacterData/DT_Quests.DT_Quests" Row)
    (:then
      (return _returnvalue))))

(fn ProgressQuest
  (params (QuestID :type Name))
  (bind _int (CallFunction|NametoInt QuestID))
  (bind _returnvalue (- _int 1))
  (bind _asgi_tiki_tandems (Utilities|Casting|CastToGI_TikiTandems (Game|GetGameInstance)))
  (Utilities|Array|SetArrayElem (Variables|/Game/Core/Blueprints/GameRules/GI_TikiTandems.GI_TikiTandems_C|GetstQuests _asgi_tiki_tandems) _returnvalue (Utilities|Struct|MakeST_Quest (.questname (Utilities|Array|Get(acopy) (Variables|/Game/Core/Blueprints/GameRules/GI_TikiTandems.GI_TikiTandems_C|GetstQuests _asgi_tiki_tandems) _returnvalue)) (.questdescription (Utilities|Array|Get(acopy) (Variables|/Game/Core/Blueprints/GameRules/GI_TikiTandems.GI_TikiTandems_C|GetstQuests _asgi_tiki_tandems) _returnvalue)) (+ (.questprogressionsteps (Utilities|Array|Get(acopy) (Variables|/Game/Core/Blueprints/GameRules/GI_TikiTandems.GI_TikiTandems_C|GetstQuests _asgi_tiki_tandems) _returnvalue)) 1) false))
  (CallFunction|ProgressWidget)
  (if (== (.questprogressionsteps (CallFunction|GetAnyQuestbyID QuestID)) (.questprogressionsteps (CallFunction|GetQuest QuestID)))
    (CallFunction|SetQuestComplete QuestID)))

(fn GetQuest
  (params (QuestID :type Name))
  (bind _asgi_tiki_tandems (Utilities|Casting|CastToGI_TikiTandems (Game|GetGameInstance)))
  (return (Utilities|Array|Get(acopy) (Variables|/Game/Core/Blueprints/GameRules/GI_TikiTandems.GI_TikiTandems_C|GetstQuests _asgi_tiki_tandems) (- (CallFunction|NametoInt QuestID) 1))))

(fn SetQuestComplete
  (params (QuestID :type Name))
  (bind _int (CallFunction|NametoInt QuestID))
  (bind _returnvalue (- _int 1))
  (bind _asgi_tiki_tandems (Utilities|Casting|CastToGI_TikiTandems (Game|GetGameInstance)))
  (Utilities|Array|SetArrayElem (Variables|/Game/Core/Blueprints/GameRules/GI_TikiTandems.GI_TikiTandems_C|GetstQuests _asgi_tiki_tandems) _returnvalue (Utilities|Struct|MakeST_Quest (.questname (Utilities|Array|Get(acopy) (Variables|/Game/Core/Blueprints/GameRules/GI_TikiTandems.GI_TikiTandems_C|GetstQuests _asgi_tiki_tandems) _returnvalue)) (.questdescription (Utilities|Array|Get(acopy) (Variables|/Game/Core/Blueprints/GameRules/GI_TikiTandems.GI_TikiTandems_C|GetstQuests _asgi_tiki_tandems) _returnvalue)) (.questprogressionsteps (Utilities|Array|Get(acopy) (Variables|/Game/Core/Blueprints/GameRules/GI_TikiTandems.GI_TikiTandems_C|GetstQuests _asgi_tiki_tandems) _returnvalue)) true)))

(fn ProgressWidget
  (bind _asbpc_training_grounds (Utilities|Casting|CastToBPC_TrainingGrounds (Game|GetPlayerController 0)))
  (Default|ProgressQuest (Variables|/Game/Core/Blueprints/Input/Controllers/BPC_TrainingGrounds.BPC_TrainingGrounds_C|GetwTrainingHUD _asbpc_training_grounds)))

(fn UpdateWidget
  (params (QuestID :type Name))
  (bind _quest (CallFunction|GetAnyQuestbyID QuestID))
  (bind (_questname _questdescription _questprogressionsteps) (Utilities|Struct|BreakST_Quest _quest))
  (bind _asbpc_training_grounds (Utilities|Casting|CastToBPC_TrainingGrounds (Game|GetPlayerController 0)))
  (Variables|/Script/UMG.WidgetSwitcher|SetActiveWidgetIndex (Variables|/Game/Core/Widgets/TrainingGrounds/W_ExplanationWidget.W_ExplanationWidget_C|GetSwitcher (Variables|/Game/Core/Blueprints/Input/Controllers/BPC_TrainingGrounds.BPC_TrainingGrounds_C|GetwExplanation _asbpc_training_grounds)) (- (CallFunction|NametoInt QuestID) 1))
  (Default|UpdateObjective (Variables|/Game/Core/Blueprints/Input/Controllers/BPC_TrainingGrounds.BPC_TrainingGrounds_C|GetwTrainingHUD _asbpc_training_grounds) _questdescription 1 _questprogressionsteps))