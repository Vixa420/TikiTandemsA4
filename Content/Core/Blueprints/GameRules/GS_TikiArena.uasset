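; GS_TikiArena is the arena match game state, coordinating start, countdown, totem progress and match end.
; Start cleanup removes cinematic actors, reveals tikis, adds controls, starts the quit-at-zero countdown and sets team overlays.
; Tick mirrors BP_WinCon's wing and fist yaw as win and power-up progress.
; Ending slows time, passes winner/loser structs to controllers and travels via GM_Arena; a polling check reports quit wins when PlayerArray empties.
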(event Custom|MC_StartGameTimer
  ;[1 1 1] Timer for match logic
  (Utilities|Time|SetTimerbyEvent (delegate Custom|UpdateGameTimer) 1.0 true))

(event Custom|UpdateGameTimer
  ;[1 1 1] Timer for match logic
  (if (== (Variables|Default|GetSeconds) 0)
    (if (== (Variables|Default|GetMinutes) 0)
      (Game|QuitGame 0 "Quit" false)
      (else
        (bind _result (Math|Integer|DecrementInt (Variables|Default|GetMinutes))
          (:%20%20
            (Variables|Default|SetMinutes _result)
            (Variables|Default|SetSeconds 59)))))
    (else
      (bind _result_2 (Math|Integer|DecrementInt (Variables|Default|GetSeconds))
        (:%20%20
          (Variables|Default|SetSeconds _result_2))))))

(event Custom|MC_AddControls
  ;[1 1 1] Add controls and startgame logic
  (for _array_element (Variables|Default|GetPlayerArray)
    (bind _asbpc_arena (Utilities|Casting|CastToBPC_Arena (Game|GetPlayerController _array_element)))
    (Default|CLAddInputs _asbpc_arena)
    (if (== (Math|Integer|%(Integer) (Variables|/Game/Core/Blueprints/Input/Controllers/BPC_Arena.BPC_Arena_C|GetiPlayerIndex _asbpc_arena) 2) 0)
      (Pawn|SetControlRotation _asbpc_arena (Math|Rotator|MakeRotator 0.0 5.0 9e+01))
      (else
        (Pawn|SetControlRotation _asbpc_arena (Math|Rotator|MakeRotator 0.0 5.0 -9e+01))))))

(event Custom|MC_SetPlayerClasses
  (params (GI_Reference :type Game%20Instance%20Object%20Reference))
  ;[1 1 1] SetPlayerClasses logic
  (bind _asgi_tiki_tandems (Utilities|Casting|CastToGI_TikiTandems GI_Reference))
  (for (_array_element _array_index) (Variables|Default|GetPlayerClasses)
    (Utilities|Array|SetArrayElem (Variables|/Game/Core/Blueprints/GameRules/GI_TikiTandems.GI_TikiTandems_C|GetPlayerClasses _asgi_tiki_tandems) _array_index _array_element)))

(event Custom|CL_SetTeamOverlay
  ;[1 1 1] Set team colors/overlay logic
  (Utilities|FlowControl|Delay 0.2)
  (for _array_element (Variables|Default|GetPlayerArray)
    (bind _asbpc_arena (Utilities|Casting|CastToBPC_Arena (Game|GetPlayerController _array_element)))
    (bind _asbp_tiki (Utilities|Casting|CastToBP_Tiki (Pawn|GetControlledPawn _asbpc_arena)))
    (Default|SRSetTeamOverlayColor _asbp_tiki (Variables|/Game/Core/Blueprints/Input/Controllers/BPC_Arena.BPC_Arena_C|GetiPlayerIndex _asbpc_arena))))

(event Custom|MC_EndTheGame
  (params (WhichTeamWon? :type E_Team%20Enum :default "NewEnumerator0"))
  ;[1 1 1] EndGame logic
  (Viewport|RemoveAllWidgets)
  (Utilities|Time|SetGlobalTimeDilation 0.2)
  (CallFunction|SetWinnerLoser WhichTeamWon?)
  (Utilities|FlowControl|Delay 1.5)
  (CallFunction|SREndScreenTravel))

(event Custom|SR_EndScreenTravel
  ;[1 1 1] EndGame logic
  (bind _asgm_arena (Utilities|Casting|CastToGM_Arena (Game|GetGameMode)))
  (Default|TraveltoEndScreen _asgm_arena))

(event Custom|StartPlayerCheck
  ;[1 1 1] PlayerLeftCheck logic
  (bind _returnvalue (Utilities|Time|SetTimerbyEvent (delegate Custom|CheckPlayers) 0.1 true)))

(event Custom|CheckPlayers
  ;[1 1 1] PlayerLeftCheck logic
  (if (and (<= (Utilities|Array|Length (Variables|Default|GetPlayerArray)) 0) (Utilities|Enum|Equal(Enum) (Variables|Default|GeteWinnerType) "NewEnumerator0"))
    (Variables|Default|SeteWinnerType "NewEnumerator1")
    (CallFunction|AnyPlayerLefttheGame)
    (Utilities|Time|ClearandInvalidateTimerbyHandle (stale Custom|StartPlayerCheck _returnvalue))))

(event Custom|AnyPlayerLeftTheGame
  ;[1 1 1] PlayerLeftCheck logic
  (bind _asgi_tiki_tandems (Utilities|Casting|CastToGI_TikiTandems (Game|GetGameInstance)))
  (Default|WinnerbyQuitting _asgi_tiki_tandems))

(event EventTick
  (params (DeltaSeconds :type Float%20%28single-precision%29))
  (bind _totem (Variables|Default|GetTotem))
  ;[1 1 1] WinCon logic
  (Variables|Default|SetWinProgress (.yaw (Variables|/Script/Engine.SceneComponent|GetRelativeRotation (Variables|/Game/Core/Blueprints/WinCondition/BP_WinCon.BP_WinCon_C|GetWingsBase _totem))))
  (Variables|Default|SetPowerUpProgress (.yaw (Variables|/Script/Engine.SceneComponent|GetRelativeRotation (Variables|/Game/Core/Blueprints/WinCondition/BP_WinCon.BP_WinCon_C|GetFistsBase _totem)))))

(event EventBeginPlay
  ;[1 1 1] BeginPlay logic
  (bind _returnvalue (Actor|GetActorOfClass "/Game/Core/Blueprints/WinCondition/BP_WinCon.BP_WinCon_C"))
  (Variables|Default|SetTotem _returnvalue))

(fn ConstructionScript)

(fn SetTotemReferences
  (bind _returnvalue (Actor|GetActorOfClass "/Game/Core/Blueprints/WinCondition/BP_WinCon.BP_WinCon_C"))
  (Variables|Default|SetWinConRef (Variables|/Game/Core/Blueprints/WinCondition/BP_WinCon.BP_WinCon_C|GetWingsBase _returnvalue))
  (Variables|Default|SetPowerUpRef (Variables|/Game/Core/Blueprints/WinCondition/BP_WinCon.BP_WinCon_C|GetFistsBase _returnvalue)))

(fn CleanupandBeginGame
  (bind _outactors (Actor|GetAllActorsOfClasswithTag "/Script/Engine.SkeletalMeshActor" "Cinematic"))
  (for _array_element _outactors
    (Actor|DestroyActor _array_element))
  (bind _outactors_2 (Actor|GetAllActorsOfClass "/Game/Core/Blueprints/TikiCharacter/Blueprint/BP_Tiki.BP_Tiki_C"))
  (for _array_element_2 _outactors_2
    (Rendering|SetActorHiddenInGame _array_element_2 false))
  (CallFunction|MCAddControls)
  (CallFunction|MCStartGameTimer)
  (CallFunction|CLSetTeamOverlay)
  (return))

(fn SetWinnerLoser
  (params (WinningTeam :type E_Team%20Enum :default "NewEnumerator0"))
  (bind _playerarray (Variables|Default|GetPlayerArray))
  (for (_array_element _array_index) _playerarray
    (bind _asbpc_arena (Utilities|Casting|CastToBPC_Arena (Game|GetPlayerController _array_element)))
    (if (Utilities|Enum|Equal(Enum) (Variables|/Game/Core/Blueprints/Input/Controllers/BPC_Arena.BPC_Arena_C|GetePlayerTeam _asbpc_arena) WinningTeam)
      (Variables|Default|SetstWinner "")
      (else
        (Variables|Default|SetstLoser (Utilities|Struct|MakeST_EndInfo (Utilities|Array|Get(acopy) (Variables|Default|GetPlayerClasses) _array_index) (Variables|/Game/Core/Blueprints/Input/Controllers/BPC_Arena.BPC_Arena_C|GetePlayerTeam _asbpc_arena))))))
  (for _array_element_2 _playerarray
    (bind _asbpc_arena_2 (Utilities|Casting|CastToBPC_Arena (Game|GetPlayerController _array_element_2)))
    (Default|CLSetEndGameStructs _asbpc_arena_2 (Variables|Default|GetstWinner) (Variables|Default|GetstLoser))
    (return)))