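; GS_Tiki is a game state that runs the match countdown and tracks progress on the totem.
; A looping one-second timer, started on BeginPlay, counts down Minutes and Seconds and quits the game when both reach zero.
; Each Tick copies the relative yaw of the BP_WinCon totem's WingsBase and FistsBase into WinProgress and PowerUpProgress, so component rotation serves as the progress value.
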(event Custom|StartGameTimer
  (Utilities|Time|SetTimerbyEvent (delegate Custom|UpdateGameTimer) 1.0 true))

(event Custom|UpdateGameTimer
  (if (== (Variables|Default|GetSeconds) 0)
    (if (== (Variables|Default|GetMinutes) 0)
      (Game|QuitGame 0 "Quit" false)
      (else
        (bind _result (Math|Integer|DecrementInt (Variables|Default|GetMinutes))
          (:%20%20
            (Variables|Default|SetMinutes _result)
            (Variables|Default|SetSeconds 59)))))
    (else
      (bind _result_2 (Math|Integer|DecrementInt (Variables|Default|GetSeconds))
        (:%20%20
          (Variables|Default|SetSeconds _result_2))))))

(event EventBeginPlay
  (bind _returnvalue (Actor|GetActorOfClass "/Game/Core/Blueprints/WinCondition/BP_WinCon.BP_WinCon_C"))
  (Variables|Default|SetTotem _returnvalue)
  (CallFunction|StartGameTimer))

(event EventTick
  (params (DeltaSeconds :type Float%20%28single-precision%29))
  (bind _totem (Variables|Default|GetTotem))
  (Variables|Default|SetWinProgress (.yaw (Variables|/Script/Engine.SceneComponent|GetRelativeRotation (Variables|/Game/Core/Blueprints/WinCondition/BP_WinCon.BP_WinCon_C|GetWingsBase _totem))))
  (Variables|Default|SetPowerUpProgress (.yaw (Variables|/Script/Engine.SceneComponent|GetRelativeRotation (Variables|/Game/Core/Blueprints/WinCondition/BP_WinCon.BP_WinCon_C|GetFistsBase _totem)))))

(fn ConstructionScript)