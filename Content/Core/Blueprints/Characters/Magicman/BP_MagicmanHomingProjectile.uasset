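; Magicman's skull projectile, which launches upward, homes in on a BP_Tiki other than its instigator and stuns Tikis it hits.
; BeginPlay targets the last matching Tiki found, while a timeline animates homing acceleration.
; Overlaps send stun duration as DT_Stun damage, then remove projectile movement, leaving the skull to physics with a sound.
; Hit VFX goes through server/multicast events, skipping spawn where the instigator is locally controlled.
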(event OnComponentBeginOverlap(Collision)
  (params (OverlappedComponent :type Primitive%20Component%20Object%20Reference) (OtherActor :type Actor%20Object%20Reference) (OtherComp :type Primitive%20Component%20Object%20Reference) (OtherBodyIndex :type Integer) (bFromSweep :type Boolean) (SweepResult :type Hit%20Result%20Structure%20%28by%20ref%29))
  (bind _returnvalue (Transformation|GetActorLocation))
  (if (and (!= OtherActor (Variables|Actor|GetInstigator)) (!= OtherComp 0))
    (Utilities|FlowControl|Sequence
      (:then_0
        (CallFunction|IfPlayerIsHit OtherActor)
        (if (Networking|IsServer)
          (CallFunction|SRVFX "/Game/Assets/VFX/Flipbook_VFX/Shared/Particles/Lightning/NS_SkullHit.NS_SkullHit" _returnvalue)
          (else
            (CallFunction|MCVFX "/Game/Assets/VFX/Flipbook_VFX/Shared/Particles/Lightning/NS_SkullHit.NS_SkullHit" _returnvalue))))
      (:then_1
        (CallFunction|IfProjectileIsHit)))))

(event Custom|MC_VFX
  (params (SystemTemplate :type Niagara%20System%20Object%20Reference) (Location :type Vector))
  (if (not (Pawn|IsLocallyControlled (Variables|Actor|GetInstigator)))
    (Niagara|SpawnSystematLocation SystemTemplate Location)))

(event Custom|SR_VFX
  (params (SystemTemplate :type Niagara%20System%20Object%20Reference) (Location :type Vector))
  (CallFunction|MCVFX SystemTemplate Location))

(event Custom|AnimateHomingStrength
  (bind _projectilemovement (Variables|Default|GetProjectileMovement))
  (bind _homingaccelerationmagnitude (Timeline|HomingStrength PlayFromStart)
    (:Update
      (Utilities|IsValid _projectilemovement
        (:Is%20Valid
          (Variables|/Script/Engine.ProjectileMovementComponent|SetHomingAccelerationMagnitude _projectilemovement _homingaccelerationmagnitude))))))

(event EventBeginPlay
  (Game|Components|ProjectileMovement|SetVelocityinLocalSpace (Variables|Default|GetProjectileMovement) "0.000000,0.000000,100.000000")
  (CallFunction|FindHomingTarget)
  (CallFunction|AnimateHomingStrength))

(fn ConstructionScript)

(fn IfPlayerIsHit
  (params (PlayerHit :type Actor%20Object%20Reference))
  (bind _asbp_tiki (Utilities|Casting|CastToBP_Tiki PlayerHit))
  (Game|Damage|ApplyDamage _asbp_tiki (Variables|Default|GetfStunDuration) 0 (Variables|Actor|GetInstigator) "/Game/Core/Data/DamageTypes/DT_Stun.DT_Stun_C"))

(fn IfProjectileIsHit
  (bind _projectilemovement (Variables|Default|GetProjectileMovement))
  (bind _skull (Variables|Default|GetSkull))
  (Utilities|IsValid _projectilemovement
    (:Is%20Valid
      (Components|DestroyComponent _projectilemovement)
      (Collision|SetCollisionEnabled _skull "PhysicsOnly")
      (Physics|SetSimulatePhysics _skull true)
      (Audio|PlaySoundatLocation "/Game/Assets/SFX/MS_ShootBasic_MM.MS_ShootBasic_MM" (Transformation|GetActorLocation) "0, 0, 0" 1.0 1.0 0.0 0 0 0 0))))

(fn FindHomingTarget
  (bind _outactors (Actor|GetAllActorsOfClass "/Game/Core/Blueprints/TikiCharacter/Blueprint/BP_Tiki.BP_Tiki_C"))
  (for _array_element _outactors
    (if (!= _array_element (Variables|Actor|GetInstigator))
      (Variables|/Script/Engine.ProjectileMovementComponent|SetHomingTargetComponent (Variables|Default|GetProjectileMovement) (Variables|/Script/Engine.Actor|GetRootComponent _array_element)))))