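; Voodooman's chakram projectile, which after a short delay homes in on the nearest BP_Tiki other than its instigator.
; Overlaps deal launch and half-strength stun damage to Tikis, pass the struck part and impact point to BP_WinCon totems for damage, or trigger training targets.
; Tiki and totem hits multicast impact VFX and sound, then destroy the projectile.
; Heavy Tiki hits also complete a training-grounds quest and raise the totem stairway.
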(event OnComponentBeginOverlap(Collision)
  (params (OverlappedComponent :type Primitive%20Component%20Object%20Reference) (OtherActor :type Actor%20Object%20Reference) (OtherComp :type Primitive%20Component%20Object%20Reference) (OtherBodyIndex :type Integer) (bFromSweep :type Boolean) (SweepResult :type Hit%20Result%20Structure%20%28by%20ref%29))
  (bind _chakram (Variables|Default|GetChakram))
  (bind _returnvalue (Transformation|GetWorldLocation _chakram))
  (if (and (!= OtherActor (Variables|Actor|GetInstigator)) (!= OtherActor self))
    (bind _asbp_tiki (Utilities|Casting|CastToBP_Tiki OtherActor)
      (:then
        (CallFunction|IfHitPlayer _asbp_tiki)
        (if (Networking|IsServer) :!label _label
          (CallFunction|SRVFX "/Game/Assets/VFX/Flipbook_VFX/Shared/Particles/Lightning/NS_ShootChakram.NS_ShootChakram" _returnvalue)
          (else
            (CallFunction|MCVFX "/Game/Assets/VFX/Flipbook_VFX/Shared/Particles/Lightning/NS_ShootChakram.NS_ShootChakram" _returnvalue))))
      (:CastFailed
        (Utilities|Casting|CastToBP_WinCon OtherActor
          (:then
            (CallFunction|IfHitTotem OtherActor OtherComp (.ImpactPoint (Collision|BreakHitResult SweepResult)))
            (goto _label))
          (:CastFailed
            (Utilities|Casting|CastToBP_Target OtherActor)
            (CallFunction|HitTarget OtherActor)))))))

(event Custom|SR_VFX
  (params (SystemTemplate :type Niagara%20System%20Object%20Reference) (Location :type Vector))
  (CallFunction|MCVFX SystemTemplate Location))

(event Custom|MC_VFX
  (params (SystemTemplate :type Niagara%20System%20Object%20Reference) (Location :type Vector))
  (Niagara|SpawnSystematLocation SystemTemplate Location)
  (Audio|PlaySoundatLocation "/Game/Assets/SFX/MS_MagicImpact.MS_MagicImpact" (Transformation|GetActorLocation) "0, 0, 0" 1.0 1.0 0.0 0 0 0 0)
  (Actor|DestroyActor))

(event EventBeginPlay
  (Utilities|FlowControl|Delay 0.5)
  (CallFunction|FindHomingTarget))

(fn ConstructionScript)

(fn IfHitPlayer
  (params (Object :type Object%20Object%20Reference))
  (bind _flaunchstrength (Variables|Default|GetfLaunchStrength))
  (bind _instigator (Variables|Actor|GetInstigator))
  (bind _asbp_tiki (Utilities|Casting|CastToBP_Tiki Object))
  (Game|Damage|ApplyDamage _asbp_tiki _flaunchstrength 0 _instigator "/Game/Core/Data/DamageTypes/DT_Launch.DT_Launch_C")
  (Game|Damage|ApplyDamage _asbp_tiki (/ _flaunchstrength 2.0) 0 _instigator "/Game/Core/Data/DamageTypes/DT_Stun.DT_Stun_C")
  (if (Variables|Default|GetbHeavy?)
    (CallFunction|HeavyAttackQuestComplete)))

(fn IfHitTotem
  (params (OtherActor :type Object%20Object%20Reference) (OtherComponent :type Primitive%20Component%20Object%20Reference) (vHitLocation :type Vector))
  (bind _collision (Variables|Default|GetCollision))
  (Utilities|IsValid _collision
    (:Is%20Valid
      (Components|DestroyComponent _collision))
    (:Is%20Not%20Valid
      _))
  (bind _asbp_win_con (Utilities|Casting|CastToBP_WinCon OtherActor))
  (Variables|/Game/Core/Blueprints/WinCondition/BP_WinCon.BP_WinCon_C|SetHitTotemPart _asbp_win_con OtherComponent)
  (Variables|/Game/Core/Blueprints/WinCondition/BP_WinCon.BP_WinCon_C|SetvHitLocation _asbp_win_con vHitLocation)
  (Utilities|FlowControl|DoOnce false
    (:Completed
      (Game|Damage|ApplyDamage _asbp_win_con (Variables|Default|GetfLaunchStrength) 0 self))))

(fn HitTarget
  (params (OtherActor :type Actor%20Object%20Reference))
  (Utilities|Casting|CastToGM_TrainingGrounds (Game|GetGameMode))
  (bind _asbp_target (Utilities|Casting|CastToBP_Target OtherActor))
  (Default|HitTarget _asbp_target))

(fn FindHomingTarget
  (Variables|Default|SetfClosestDistance 2e+09)
  (bind _outactors (Actor|GetAllActorsOfClass "/Game/Core/Blueprints/TikiCharacter/Blueprint/BP_Tiki.BP_Tiki_C"))
  (for (_array_element _array_index) _outactors
    (if (!= _array_element (Variables|Actor|GetInstigator))
      (if (< (Math|Vector|Distance(Vector) (Transformation|GetActorLocation _array_element) (Transformation|GetWorldLocation (Variables|Default|GetChakram))) (Variables|Default|GetfClosestDistance))
        (LocalVariables|SetiNearestIndex _array_index)
        (Variables|Default|SetfClosestDistance (Math|Vector|Distance(Vector) (Transformation|GetActorLocation _array_element) (Transformation|GetWorldLocation (Variables|Default|GetChakram)))))))
  (Variables|/Script/Engine.ProjectileMovementComponent|SetHomingTargetComponent (Variables|Default|GetProjectileMovement) (Variables|/Script/Engine.Actor|GetRootComponent (Utilities|Array|Get(acopy) _outactors (LocalVariables|GetiNearestIndex)))))

(fn HeavyAttackQuestComplete
  (Utilities|FlowControl|DoOnce false
    (:Completed
      (Utilities|Casting|CastToGM_TrainingGrounds (Game|GetGameMode))
      (CallFunction|ProgressWidget)
      (CallFunction|SetQuestComplete "6")
      (bind _returnvalue (Actor|GetActorOfClass "/Game/Core/Blueprints/Obstacles/BP_TotemRoundStairway.BP_TotemRoundStairway_C"))
      (Default|BringUpStairs _returnvalue))))