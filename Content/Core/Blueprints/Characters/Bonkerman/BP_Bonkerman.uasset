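; Bonkerman, a playable bat-wielding character with basic, heavy and special attacks, replicated mostly through server-to-multicast events.
; A recharging energy bar gates attacks and scales bat-throw velocity and swing speed.
; Heavy swings re-trace from the weapon socket during the montage, launching BP_Tiki targets twice, then stunning on the third hit.
; The special is a timed rage granting stun release, invincibility, speed and free attacks, with training-grounds quest hooks.
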(event Custom|ResetOnUnStunned
  ;[1 1 1] Event BeginPlay
  (Variables|/Script/Engine.CharacterMovementComponent|SetMaxWalkSpeed (Variables|Character|GetCharacterMovement) (Variables|Default|GetfBonkerWalkSpeed)))

(event Custom|MC_Recharge
  ;[1 1 1] Event BeginPlay
  (CallFunction|AddEnergy))

(event Custom|MC_PlayBasicAttackAnimation
  (params (eState :type E_State%20Enum :default "NewEnumerator0"))
  ;[0 1 0.06274] BasicAttack
  (if (not (Pawn|IsLocallyControlled (Variables|Default|GetInstigator)))
    (Animation|Montage|PlayMontage (Variables|Character|GetMesh) "/Game/Assets/TikiCharacter/Animations/Bonkerman/AM_BatThrow.AM_BatThrow"
      (:OnBlendOut
        (Variables|Default|SeteState eState)))))

(event Custom|SR_PlayBasicAttackAnimation
  (params (eState :type E_State%20Enum :default "NewEnumerator0"))
  ;[0 1 0.06274] BasicAttack
  (CallFunction|MCPlayBasicAttackAnimation eState))

(event Custom|MC_PlaySpecialAttackAnimation
  ;[1 0.02353 0] SpecialAttack
  (Animation|Montage|PlayMontage (Variables|Character|GetMesh) "/Game/Assets/TikiCharacter/Animations/Bonkerman/AM_GetRaged.AM_GetRaged"
    (:OnNotifyBegin
      (Variables|Default|SeteState "NewEnumerator0")
      (CallFunction|Enrage)
      (bind _returnvalue (Utilities|Time|SetTimerbyEvent (delegate Custom|DisableRage) (Variables|Default|GetfRageDuration))))))

(event Custom|SR_PlaySpecialAttackAnimation
  ;[1 0.02353 0] SpecialAttack
  (CallFunction|MCPlaySpecialAttackAnimation))

(event Custom|DisableRage
  ;[1 0.02353 0] SpecialAttack
  (CallFunction|SRDisableRage))

(event Custom|MC_DisableRage
  ;[1 0.02353 0] SpecialAttack
  (CallFunction|Unrage)
  (Utilities|Time|ClearandInvalidateTimerbyHandle (stale Custom|MC_PlaySpecialAttackAnimation _returnvalue)))

(event Custom|SR_DisableRage
  ;[1 0.02353 0] SpecialAttack
  (CallFunction|MCDisableRage))

(event Custom|SR_Recharge
  ;[1 1 1] Event BeginPlay
  (CallFunction|MCRecharge))

(event Custom|MC_HeavyAttack
  (params (fChargeBarValue :type Float%20%28double-precision%29))
  ;[0 1 0.8588] HeavyAttack
  (bind _notifyname (Animation|Montage|PlayMontage (Variables|Character|GetMesh) "/Game/Assets/TikiCharacter/Animations/Bonkerman/AM_BatHit.AM_BatHit" (Math|Float|Clamp(Float) (* fChargeBarValue 2.0) 0.5 1.6))
    (:OnBlendOut
      (if (Utilities|Enum|NotEqual(Enum) (Variables|Default|GeteState) "NewEnumerator3")
        (Variables|Default|SeteState "NewEnumerator0")))
    (:OnNotifyBegin
      (if (== _notifyname "Start")
        (CallFunction|TraceLogic)
        (Variables|Default|SetbShouldTrace? true)
        (CallFunction|ResetHeavyDamage)
        (else
          (Variables|Default|SetbShouldTrace? false))))))

(event Custom|SR_HeavyAttack
  (params (EnergyCost :type Float%20%28double-precision%29) (fChargeBarValue :type Float%20%28double-precision%29))
  ;[0 1 0.8588] HeavyAttack
  (CallFunction|MCHeavyAttack fChargeBarValue)
  (CallFunction|CLUseEnergy EnergyCost))

(event Custom|MC_SpawnNormalProjectile
  (params (Class :type BP%20Bat%20Projectile%20Class%20Reference) (SpawnTransform :type Transform) (CollisionHandlingOverride :type ESpawnActorCollisionHandlingMethod%20Enum :default "Undefined") (Owner :type Actor%20Object%20Reference) (Instigator :type Pawn%20Object%20Reference) (fLaunchStrength :type Float%20%28double-precision%29) (NewVelocity :type Vector))
  ;[0 1 0.06274] BasicAttack
  (bind _returnvalue (Game|SpawnActorfromClass Class SpawnTransform CollisionHandlingOverride "MultiplyWithRoot" Owner Instigator))
  (Variables|/Game/Core/Blueprints/Characters/Bonkerman/BP_BatProjectile.BP_BatProjectile_C|SetfLaunchStrength _returnvalue fLaunchStrength)
  (Game|Components|ProjectileMovement|SetVelocityinLocalSpace (Variables|/Game/Core/Blueprints/Characters/Bonkerman/BP_BatProjectile.BP_BatProjectile_C|GetProjectileMovement _returnvalue) NewVelocity))

(event Custom|SR_SpawnNormalProjectile
  (params (Class :type BP%20Bat%20Projectile%20Class%20Reference) (SpawnTransform :type Transform) (CollisionHandlingOverride :type ESpawnActorCollisionHandlingMethod%20Enum :default "Undefined") (Owner :type Actor%20Object%20Reference) (Instigator :type Pawn%20Object%20Reference) (fLaunchStrength :type Float%20%28double-precision%29) (NewVelocity :type Vector))
  ;[0 1 0.06274] BasicAttack
  (CallFunction|MCSpawnNormalProjectile Class SpawnTransform CollisionHandlingOverride Owner Instigator fLaunchStrength NewVelocity))

(event Custom|CL_UseEnergy
  (params (EnergyCost :type Float%20%28double-precision%29))
  ;[1 1 1] Event BeginPlay
  (CallFunction|UseEnergy EnergyCost))

(event Custom|TraceLogic
  (bind (_start _end _ignore) (Utilities|TracingData))
  ;[0 1 0.8588] HeavyAttack
  (bind (_outhit _returnvalue) (Collision|LineTraceByChannel _start _end "TraceTypeQuery1" false _ignore "None"))
  (if _returnvalue
    (if (Actor|ActorHasTag (.HitActor (Collision|BreakHitResult _outhit)) "Character")
      (if (Networking|IsServer)
        (CallFunction|SRTraceDamage false (.ImpactPoint (Collision|BreakHitResult _outhit)) (.HitActor (Collision|BreakHitResult _outhit)))
        (else
          (CallFunction|MCTraceDamage false (.ImpactPoint (Collision|BreakHitResult _outhit)) (.HitActor (Collision|BreakHitResult _outhit)))))
      (else
        (Utilities|FlowControl|Delay 0.001)
        (if (Variables|Default|GetbShouldTrace?)
          (CallFunction|TraceLogic))))))

(event Custom|ResetHeavyDamage
  (bind _returnvalue (Pawn|GetController))
  (bind _instigator (Variables|Default|GetInstigator))
  (bind _character_info (Variables|Default|GetCharacter%20Info))
  (bind _heavyabillity (Utilities|Struct|BreakST_CharacterInfo _character_info))
  (bind _damage (Utilities|Struct|BreakST_AbillityInfo _heavyabillity))
  ;[0 1 0.8588] HeavyAttack
  (Utilities|FlowControl|DoOnce false) ; enters at Reset
)

(event Custom|MC_TraceDamage
  (params (bShouldTrace? :type Boolean) (Location :type Vector) (Object :type Object%20Object%20Reference))
  (bind _returnvalue (Pawn|GetController))
  (bind _instigator (Variables|Default|GetInstigator))
  (bind _character_info (Variables|Default|GetCharacter%20Info))
  (bind _heavyabillity (Utilities|Struct|BreakST_CharacterInfo _character_info))
  (bind _damage (Utilities|Struct|BreakST_AbillityInfo _heavyabillity))
  ;[0 1 0.8588] HeavyAttack
  (Variables|Default|SetbShouldTrace? bShouldTrace?)
  (CallFunction|HeavyVFX "/Game/Assets/VFX/Flipbook_VFX/Shared/Particles/Dust/NS_SmallDustHit.NS_SmallDustHit" Location)
  (bind _asbp_tiki (Utilities|Casting|CastToBP_Tiki Object))
  (Utilities|FlowControl|DoOnce false
    (:Completed
      (switch int (Variables|Default|GetiCounter)
        (:0
          (Game|Damage|ApplyDamage _asbp_tiki (/ _damage 2.5) 0 _instigator "/Game/Core/Data/DamageTypes/DT_Launch.DT_Launch_C" :!label _label)
          (Math|Integer|IncrementInt (Variables|Default|GetiCounter)
            (:%20%20
              (CallFunction|HeavyAttackQuestComplete)
              (Class|BPIEIK|Bonks(Message) _returnvalue))))
        (:1
          (goto _label))
        (:2
          (Game|Damage|ApplyDamage _asbp_tiki _damage 0 _instigator "/Game/Core/Data/DamageTypes/DT_Stun.DT_Stun_C")
          (Variables|Default|SetiCounter 0)
          (Class|BPIEIK|Bonks(Message) _returnvalue))))))

(event Custom|SR_TraceDamage
  (params (bShouldTrace? :type Boolean) (Location :type Vector) (Object :type Object%20Object%20Reference))
  ;[0 1 0.8588] HeavyAttack
  (CallFunction|MCTraceDamage bShouldTrace? Location Object))

(event Custom|TryAgainTraining
  ;[1 1 1] Event BeginPlay
  (Utilities|FlowControl|Delay 3.0)
  (if (Variables|Default|GetbQuestDone?)
    (CallFunction|SpecialAttackQuestComplete)
    (CallFunction|CloseGate)
    (else
      (CallFunction|SpecialAttackQuestFailed))))

(event Custom|TimerRecharge
  ;[1 1 1] Event BeginPlay
  (if (Networking|IsServer)
    (CallFunction|SRRecharge)
    (else
      (CallFunction|MCRecharge))))

(event Custom|CloseGate
  ;[1 0.02353 0] SpecialAttack
  (Utilities|FlowControl|Gate false) ; enters at Close
)

(event Custom|BasicAttackStarted
  (bind (_projectiletransform _owner _self _launchstrength _velocity) (Utilities|ProjectileData))
  ;[0 1 0.06274] BasicAttack
  (if (Utilities|CanNormalAttackwithEnergy?)
    (Utilities|FlowControl|Sequence
      (:then_0
        (Animation|Montage|PlayMontage (Variables|Character|GetMesh) "/Game/Assets/TikiCharacter/Animations/Bonkerman/AM_BatThrow.AM_BatThrow"
          (:OnBlendOut
            (if (Utilities|Enum|Equal(Enum) (Variables|Default|GeteState) "NewEnumerator3")
              (CallFunction|SRDisableRage))
            (Variables|Default|SeteState "NewEnumerator0"))
          (:OnNotifyBegin
            (CallFunction|SRSpawnNormalProjectile "/Game/Core/Blueprints/Characters/Bonkerman/BP_BatProjectile.BP_BatProjectile_C" _projectiletransform "AlwaysSpawn" _owner _self _launchstrength _velocity)
            (CallFunction|CLUseEnergy (Variables|Default|GetfBasicAttackCost)))))
      (:then_1
        (CallFunction|SRPlayBasicAttackAnimation "NewEnumerator0")))))

(event Custom|HeavyAttackStarted
  ;[0 1 0.8588] HeavyAttack
  (if (Utilities|CanHeavyAttackwithEnergy?)
    (Variables|Default|SetbIsHeavyAttackOnCD true)
    (CallFunction|SRHeavyAttack (Variables|Default|GetfHeavyAttackCost) (Variables|Default|GetfChargebarValue))))

(event Custom|SpecialAttackStarted
  ;[1 0.02353 0] SpecialAttack
  (if (not (Variables|Default|GetbIsSpecialAttackOnCD))
    (CallFunction|SRPlaySpecialAttackAnimation)
    (Variables|Default|SetbIsSpecialAttackOnCD true)
    (Utilities|FlowControl|Gate false
      (:Exit
        (Utilities|StunCheckLogic)))))

(event EventICBasicAttackStarted
  ;[1 1 1] CombatInterfaceEvents
  (CallFunction|BasicAttackStarted))

(event EventICHeavyAttackStarted
  ;[1 1 1] CombatInterfaceEvents
  (CallFunction|HeavyAttackStarted))

(event EventICSpecialAttackStarted
  ;[1 1 1] CombatInterfaceEvents
  (CallFunction|SpecialAttackStarted))

(event EventBeginPlay
  ;[1 1 1] Event BeginPlay
  (|CallParentFunction)
  (Utilities|Time|SetTimerbyEvent (delegate Custom|TimerRecharge) (Variables|Default|GetfRefreshTimer) true)
  (EventDispatchers|BindEventtoOnUnStunned (delegate Custom|ResetOnUnStunned))
  (Variables|Default|SetfRageDuration (Utilities|Struct|BreakST_AbillityInfo (.SpecialAbillity (Utilities|Struct|BreakST_CharacterInfo (Variables|Default|GetCharacter%20Info)))))
  (Utilities|Casting|CastToGM_TrainingGrounds (Game|GetGameMode))
  (EventDispatchers|BindEventtoOnStunned (delegate Custom|TryAgainTraining)))

(fn ConstructionScript
  (Variables|Default|SeteCharacterClass "NewEnumerator1")
  (|CallParentFunction))

(fn AddEnergy
  (if (< (Variables|Default|GetfChargebarValue) 1.0)
    (Variables|Default|SetfCurrentRefreshSpeed (+ (Variables|Default|GetfCurrentRefreshSpeed) 0.002))
    (Variables|Default|SetfChargebarValue (+ (Variables|Default|GetfChargebarValue) (/ (Variables|Default|GetfRefreshTimer) (/ 1.0 (Variables|Default|GetfCurrentRefreshSpeed)))))))

(fn Enrage
  (Variables|Default|SetbQuestDone? true)
  (Default|CallOnUnStunned)
  (Variables|Default|SeteState "NewEnumerator3")
  (CallFunction|UnStun)
  (Networking|SwitchHasAuthority
    (:Authority
      (CallFunction|MCUnstunned))
    (:Remote
      (CallFunction|SRUnstunned)))
  (Variables|Default|SetfChargebarValue 1.0)
  (Variables|/Script/Engine.CharacterMovementComponent|SetMaxWalkSpeed (Variables|Character|GetCharacterMovement) (Variables|Default|GetfEnragedMoveSpeed))
  (Variables|Default|SetbIsInvincible? true)
  (Audio|SpawnSoundatLocation "/Game/Assets/SFX/MS_Roar.MS_Roar" (Transformation|GetActorLocation) "0, 0, 0" 1.0 1.0 0.0 0 0)
  (Development|SetHiddeninGame (Variables|Default|GetVFX) false false)
  (return))

(fn Unrage
  (Variables|Default|SetbIsInvincible? false)
  (Variables|/Script/Engine.CharacterMovementComponent|SetMaxWalkSpeed (Variables|Character|GetCharacterMovement) (Variables|Default|GetfBonkerWalkSpeed))
  (Development|SetHiddeninGame (Variables|Default|GetVFX) true false)
  (Variables|Default|SeteState "NewEnumerator0"))

(fn UseEnergy
  (params (EnergyCost :type Float%20%28double-precision%29))
  (if (not (Utilities|Enum|Equal(Enum) (Variables|Default|GeteState) "NewEnumerator3"))
    (Variables|Default|SetfChargebarValue (- (Variables|Default|GetfChargebarValue) EnergyCost))
    (Variables|Default|SetfCurrentRefreshSpeed (Variables|Default|GetfDefaultRefreshSpeed))))

(fn HeavyVFX
  (params (SystemTemplate :type Niagara%20System%20Object%20Reference) (Location :type Vector))
  (Niagara|SpawnSystematLocation SystemTemplate Location)
  (Audio|SpawnSoundatLocation "/Game/Assets/SFX/MS_FootSteps.MS_FootSteps" (Transformation|GetActorLocation) "0, 0, 0" 1.0 1.0 0.0 0 0))