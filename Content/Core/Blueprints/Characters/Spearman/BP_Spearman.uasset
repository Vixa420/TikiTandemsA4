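; Spearman player class Blueprint with three combat-interface attacks: a charged spear throw, a heavy stun strike and a special throw.
; Basic charge time sets projectile launch strength, velocity and gravity, while the special holds an idle pose until released at full strength.
; Heavy attack line-traces from the weapon socket on a montage notify, applying stun damage to characters.
; An EState enum gates attacks, and SR/MC event pairs replicate montages, traces and projectile spawns.
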(event Custom|ResetOnUnStunned
  ;[1 1 1] EventBeginPlay
  (Variables|/Script/Engine.CharacterMovementComponent|SetMaxWalkSpeed (Variables|Character|GetCharacterMovement) (Variables|Default|GetfDefaultWalkSpeed)))

(event Custom|TryAgainTraining
  ;[1 1 1] EventBeginPlay
  (CallFunction|SpecialAttackQuestFailed))

(event Custom|SpecialAttackStarted
  ;[1 0.02353 0] SpecialAttack
  (if (|CanUseSpecialAttack)
    (Variables|Default|SetbIsSpecialAttackOnCD true)
    (CallFunction|SRSpecialAttackAnimation "NewEnumerator1" "NewEnumerator3" 0.0)))

(event Custom|BasicAttackTriggered
  (params (ElapsedSeconds :type Float%20%28double-precision%29))
  ;[0 1 0.06274] BasicAttack
  (if (not (Variables|Default|GetbCanAttack?))
    (Utilities|FlowControl|Gate true
      (:Exit
        (if (<= ElapsedSeconds (Variables|Default|GetfMaxChargeTime))
          (Variables|Default|SetfChargebarValue ElapsedSeconds))))))

(event Custom|BasicAttackStarted
  (bind (_spearprojectiletransform _owner _self _launchstrength _gravityscale _velocity) (Utilities|ProjectileData))
  ;[0 1 0.06274] BasicAttack
  (if (Utilities|Enum|Equal(Enum) (Variables|Default|GeteState) "NewEnumerator0")
    (Utilities|FlowControl|Sequence
      (:then_0
        (Variables|Default|SeteState "NewEnumerator1")
        (CallFunction|SRPlayStartAttackAnimation (Variables|Default|GetfMaxChargeTime)))
      (:then_1
        (Utilities|FlowControl|DoOnce false) ; enters at Reset
      ))))

(event Custom|BasicAttackCompleted
  ;[0 1 0.06274] BasicAttack
  (if (Utilities|Enum|Equal(Enum) (Variables|Default|GeteState) "NewEnumerator3")
    (CallFunction|FireSpecialAttack)
    (else
      (CallFunction|FinishAttack))))

(event Custom|HeavyAttackStarted
  ;[0 1 0.8588] HeavyAttack
  (if (|CanUseHeavyAttack)
    (Variables|Default|SetbIsHeavyAttackOnCD true)
    (CallFunction|SRHeavyAttack)))

(event Custom|OpenChargeGate
  ;[0 1 0.06274] BasicAttack
  (Utilities|FlowControl|Gate true) ; enters at Open
)

(event Custom|CloseChargeGate
  ;[0 1 0.06274] BasicAttack
  (Utilities|FlowControl|Gate true) ; enters at Close
)

(event Custom|FinishAttack
  (bind (_spearprojectiletransform _owner _self _launchstrength _gravityscale _velocity) (Utilities|ProjectileData))
  ;[0 1 0.06274] BasicAttack
  (Utilities|FlowControl|DoOnce false
    (:Completed
      (Variables|Default|SetfLaunchStrength (Math|Float|NormalizetoRange (Variables|Default|GetfChargebarValue) 0.0 (Variables|Default|GetfMaxChargeTime)))
      (Variables|Default|SetfChargebarValue 0.0)
      (if (Utilities|Enum|Equal(Enum) (Variables|Default|GeteState) "NewEnumerator1")
        (Utilities|FlowControl|Sequence
          (:then_0
            (Animation|Montage|PlayMontage (Variables|Character|GetMesh) "/Game/Assets/TikiCharacter/Animations/Spearman/AM_SpearmanBasicFire.AM_SpearmanBasicFire"
              (:then
                (CallFunction|CloseChargeGate))
              (:OnNotifyBegin
                (bind _output_get (Variables|Default|SeteState "NewEnumerator0"))
                (CallFunction|SRSpawnNormalProjectile "/Game/Core/Blueprints/Characters/Spearman/BP_SpearProjectile.BP_SpearProjectile_C" _spearprojectiletransform "AlwaysSpawn" _owner _self _launchstrength _gravityscale _velocity _output_get))))
          (:then_1
            (CallFunction|SRPlayBasicFireAttackAnimation "NewEnumerator0")))))))

(event Custom|MC_PlayStartAttackAnimation
  (params (PlayRate :type Float%20%28single-precision%29))
  (bind _mesh (Variables|Character|GetMesh))
  ;[0 1 0.06274] BasicAttack
  (CallFunction|OpenChargeGate)
  (Animation|Montage|PlayMontage _mesh "/Game/Assets/TikiCharacter/Animations/Spearman/AM_StartBasicAttack.AM_StartBasicAttack" PlayRate
    (:then
      (CallFunction|SlowDownAim))
    (:OnBlendOut
      (Animation|Montage|PlayMontage _mesh "/Game/Assets/TikiCharacter/Animations/Spearman/AM_HoldSpear.AM_HoldSpear"))))

(event Custom|SR_PlayStartAttackAnimation
  (params (PlayRate :type Float%20%28single-precision%29))
  ;[0 1 0.06274] BasicAttack
  (CallFunction|MCPlayStartAttackAnimation PlayRate))

(event Custom|SR_PlayBasicFireAttackAnimation
  (params (eState :type E_State%20Enum :default "NewEnumerator0"))
  ;[0 1 0.06274] BasicAttack
  (CallFunction|MCPlayBasicFireAttackAnimation eState))

(event Custom|MC_PlayBasicFireAttackAnimation
  (params (eState :type E_State%20Enum :default "NewEnumerator0"))
  ;[0 1 0.06274] BasicAttack
  (if (not (Pawn|IsLocallyControlled (Variables|Default|GetInstigator)))
    (Animation|Montage|PlayMontage (Variables|Character|GetMesh) "/Game/Assets/TikiCharacter/Animations/Spearman/AM_SpearmanBasicFire.AM_SpearmanBasicFire"
      (:OnBlendOut
        (Variables|Default|SeteState eState)))))

(event Custom|SR_SpawnSpecialProjectile
  (params (Class :type BP%20Spear%20Projectile%20Class%20Reference) (SpawnTransform :type Transform) (CollisionHandlingOverride :type ESpawnActorCollisionHandlingMethod%20Enum :default "Undefined") (Owner :type Actor%20Object%20Reference) (Instigator :type Pawn%20Object%20Reference) (LaunchStrength :type Float%20%28double-precision%29) (ProjectileGravityScale :type Float%20%28double-precision%29) (Velocity :type Vector))
  ;[1 0.02353 0] SpecialAttack
  (CallFunction|MCSpawnSpecialProjectile Class SpawnTransform CollisionHandlingOverride Owner Instigator LaunchStrength ProjectileGravityScale Velocity))

(event Custom|MC_SpawnSpecialProjectile
  (params (Class :type BP%20Spear%20Projectile%20Class%20Reference) (SpawnTransform :type Transform) (CollisionHandlingOverride :type ESpawnActorCollisionHandlingMethod%20Enum :default "Undefined") (Owner :type Actor%20Object%20Reference) (Instigator :type Pawn%20Object%20Reference) (LaunchStrength :type Float%20%28double-precision%29) (ProjectileGravityScale :type Float%20%28double-precision%29) (Velocity :type Vector))
  ;[1 0.02353 0] SpecialAttack
  (bind _returnvalue (Game|SpawnActorfromClass Class SpawnTransform CollisionHandlingOverride "MultiplyWithRoot" Owner Instigator))
  (Variables|/Game/Core/Blueprints/Characters/Spearman/BP_SpearProjectile.BP_SpearProjectile_C|SetfLaunchStrength _returnvalue LaunchStrength)
  (Game|Components|ProjectileMovement|SetVelocityinLocalSpace (Variables|/Game/Core/Blueprints/Characters/Spearman/BP_SpearProjectile.BP_SpearProjectile_C|GetProjectileMovement _returnvalue) Velocity)
  (Variables|/Script/Engine.ProjectileMovementComponent|SetProjectileGravityScale (Variables|/Game/Core/Blueprints/Characters/Spearman/BP_SpearProjectile.BP_SpearProjectile_C|GetProjectileMovement _returnvalue) ProjectileGravityScale)
  (Variables|/Game/Core/Blueprints/Characters/Spearman/BP_SpearProjectile.BP_SpearProjectile_C|SetbIsSpecial? _returnvalue true))

(event Custom|MC_HeavyAttack
  ;[0 1 0.8588] HeavyAttack
  (Animation|Montage|PlayMontage (Variables|Character|GetMesh) "/Game/Assets/TikiCharacter/Animations/Spearman/AM_Spearman_HeavyAttack.AM_Spearman_HeavyAttack"
    (:then
      (Variables|Default|SeteState "NewEnumerator2"))
    (:OnCompleted
      (Variables|Default|SeteState "NewEnumerator0"))
    (:OnNotifyBegin
      (Variables|Default|SetbShouldTrace? false)
      (CallFunction|SRTraceandDamage))))

(event Custom|SR_HeavyAttack
  ;[0 1 0.8588] HeavyAttack
  (CallFunction|MCHeavyAttack))

(event Custom|MC_TraceAndDamage
  (params (Start :type Vector) (End :type Vector) (ObjectTypes :type Array%20of%20EObjectTypeQuery%20Enums :default "ObjectTypeQuery1"))
  ;[0 1 0.8588] HeavyAttack
  (bind (_outhit _returnvalue) (Collision|LineTraceForObjects Start End ObjectTypes false 0 "None"))
  (if _returnvalue
    (if (Actor|ActorHasTag (.HitActor (Collision|BreakHitResult _outhit)) "Character")
      (Game|Damage|ApplyDamage (.HitActor (Collision|BreakHitResult _outhit)) (Variables|Default|GetfHeavyAttackStunDuration) 0 (Variables|Default|GetInstigator) "/Game/Core/Data/DamageTypes/DT_Stun.DT_Stun_C")
      (Audio|SpawnSound2D "/Game/Assets/SFX/MS_BloodIMpact.MS_BloodIMpact" 1.0 1.0 0.0 0)
      (Niagara|SpawnSystematLocation "/Game/Assets/VFX/Flipbook_VFX/Shared/Particles/Dust/NS_DustHit.NS_DustHit" (.ImpactPoint (Collision|BreakHitResult _outhit)))
      (CallFunction|HeavyAttackQuestComplete)
      (else
        (Utilities|FlowControl|Delay 0.03)
        (if (Variables|Default|GetbShouldTrace?)
          (CallFunction|SRTraceandDamage))))))

(event Custom|SR_TraceAndDamage
  (bind (_start _end _objecttypes) (Utilities|TraceData))
  ;[0 1 0.8588] HeavyAttack
  (CallFunction|MCTraceandDamage _start _end _objecttypes)
  (Utilities|FlowControl|Delay 0.2)
  (Variables|Default|SetbShouldTrace? false))

(event Custom|MC_SpecialAttackAnimation
  (params (FirstState :type E_State%20Enum :default "NewEnumerator0") (StateOnBlendOut :type E_State%20Enum :default "NewEnumerator0") (fChargebarValue :type Float%20%28double-precision%29))
  (bind _mesh (Variables|Character|GetMesh))
  ;[1 0.02353 0] SpecialAttack
  (Variables|Default|SeteState FirstState)
  (Animation|Montage|PlayMontage _mesh "/Game/Assets/TikiCharacter/Animations/Spearman/AM_SpearmanSpecial.AM_SpearmanSpecial"
    (:OnBlendOut
      (Variables|Default|SeteState StateOnBlendOut)
      (Animation|Montage|PlayMontage _mesh "/Game/Assets/TikiCharacter/Animations/Spearman/AM_SpearmanSpecialIdle.AM_SpearmanSpecialIdle"
        (:then
          (Variables|Default|SetfChargebarValue fChargebarValue))))))

(event Custom|SR_SpecialAttackAnimation
  (params (FirstState :type E_State%20Enum :default "NewEnumerator0") (StateOnBlendOut :type E_State%20Enum :default "NewEnumerator0") (fChargebarValue :type Float%20%28double-precision%29))
  ;[1 0.02353 0] SpecialAttack
  (CallFunction|MCSpecialAttackAnimation FirstState StateOnBlendOut fChargebarValue))

(event Custom|FireSpecialAttack
  (bind (_spearprojectiletransform _owner _self _launchstrength _gravityscale _velocity) (Utilities|ProjectileData))
  ;[1 0.02353 0] SpecialAttack
  (Variables|Default|SetfDamageMultiplier 1.0)
  (Variables|Default|SetfLaunchStrength (Variables|Default|GetfMaxChargeTime))
  (Utilities|FlowControl|Sequence
    (:then_0
      (Animation|Montage|PlayMontage (Variables|Character|GetMesh) "/Game/Assets/TikiCharacter/Animations/Spearman/AM_SpearmanSpecial_Throw.AM_SpearmanSpecial_Throw"
        (:OnBlendOut
          (CallFunction|FinishAttack)
          (Variables|Default|SeteState "NewEnumerator0")
          (Variables|Default|SetfChargebarValue 0.0))
        (:OnNotifyBegin
          (CallFunction|SRSpawnSpecialProjectile "/Game/Core/Blueprints/Characters/Spearman/BP_SpearProjectile.BP_SpearProjectile_C" _spearprojectiletransform "AlwaysSpawn" _owner _self _launchstrength _gravityscale _velocity))))
    (:then_1
      (CallFunction|SRPlaySpecialFireAttackAnimation "NewEnumerator0"))))

(event Custom|MC_PlaySpecialFireAttackAnimation
  (params (StateOnBlendOut :type E_State%20Enum :default "NewEnumerator0"))
  ;[1 0.02353 0] SpecialAttack
  (if (not (Pawn|IsLocallyControlled (Variables|Default|GetInstigator)))
    (Animation|Montage|PlayMontage (Variables|Character|GetMesh) "/Game/Assets/TikiCharacter/Animations/Spearman/AM_SpearmanSpecial_Throw.AM_SpearmanSpecial_Throw"
      (:OnBlendOut
        (Variables|Default|SeteState StateOnBlendOut)))))

(event Custom|SR_PlaySpecialFireAttackAnimation
  (params (StateOnBlendOut :type E_State%20Enum :default "NewEnumerator0"))
  ;[1 0.02353 0] SpecialAttack
  (CallFunction|MCPlaySpecialFireAttackAnimation StateOnBlendOut))

(event Custom|SR_SpawnNormalProjectile
  (params (Class :type BP%20Spear%20Projectile%20Class%20Reference) (SpawnTransform :type Transform) (CollisionHandlingOverride :type ESpawnActorCollisionHandlingMethod%20Enum :default "Undefined") (Owner :type Actor%20Object%20Reference) (Instigator :type Pawn%20Object%20Reference) (LaunchStrength :type Float%20%28double-precision%29) (ProjectileGravityScale :type Float%20%28double-precision%29) (Velocity :type Vector) (State :type E_State%20Enum :default "NewEnumerator0"))
  ;[0 1 0.06274] BasicAttack
  (CallFunction|MCSpawnNormalProjectile Class SpawnTransform CollisionHandlingOverride Owner Instigator LaunchStrength ProjectileGravityScale Velocity State))

(event Custom|MC_SpawnNormalProjectile
  (params (Class :type BP%20Spear%20Projectile%20Class%20Reference) (SpawnTransform :type Transform) (CollisionHandlingOverride :type ESpawnActorCollisionHandlingMethod%20Enum :default "Undefined") (Owner :type Actor%20Object%20Reference) (Instigator :type Pawn%20Object%20Reference) (LaunchStrength :type Float%20%28double-precision%29) (ProjectileGravityScale :type Float%20%28double-precision%29) (Velocity :type Vector) (State :type E_State%20Enum :default "NewEnumerator0"))
  ;[0 1 0.06274] BasicAttack
  (Variables|Default|SeteState State)
  (bind _returnvalue (Game|SpawnActorfromClass Class SpawnTransform CollisionHandlingOverride "MultiplyWithRoot" Owner Instigator))
  (Variables|/Game/Core/Blueprints/Characters/Spearman/BP_SpearProjectile.BP_SpearProjectile_C|SetfLaunchStrength _returnvalue LaunchStrength)
  (Game|Components|ProjectileMovement|SetVelocityinLocalSpace (Variables|/Game/Core/Blueprints/Characters/Spearman/BP_SpearProjectile.BP_SpearProjectile_C|GetProjectileMovement _returnvalue) Velocity)
  (Variables|/Script/Engine.ProjectileMovementComponent|SetProjectileGravityScale (Variables|/Game/Core/Blueprints/Characters/Spearman/BP_SpearProjectile.BP_SpearProjectile_C|GetProjectileMovement _returnvalue) ProjectileGravityScale))

(event EventICBasicAttackCompleted
  ;[1 1 1] CombatInterfaceEvents
  (CallFunction|BasicAttackCompleted))

(event EventICBasicAttackStarted
  ;[1 1 1] CombatInterfaceEvents
  (CallFunction|BasicAttackStarted))

(event EventICBasicAttackTriggered
  (params (ElapsedSeconds :type Float%20%28double-precision%29))
  ;[1 1 1] CombatInterfaceEvents
  (CallFunction|BasicAttackTriggered ElapsedSeconds))

(event EventICHeavyAttackStarted
  ;[1 1 1] CombatInterfaceEvents
  (CallFunction|HeavyAttackStarted))

(event EventICSpecialAttackStarted
  ;[1 1 1] CombatInterfaceEvents
  (CallFunction|SpecialAttackStarted))

(event EventBeginPlay
  ;[1 1 1] EventBeginPlay
  (|CallParentFunction)
  (EventDispatchers|BindEventtoOnUnStunned (delegate Custom|ResetOnUnStunned))
  (Variables|Default|SetfHeavyAttackStunDuration (Utilities|Struct|BreakST_AbillityInfo (.HeavyAbillity (Utilities|Struct|BreakST_CharacterInfo (Variables|Default|GetCharacter%20Info)))))
  (EventDispatchers|BindEventtoOnStunned (delegate Custom|TryAgainTraining)))

(fn ConstructionScript
  (Variables|Default|SeteCharacterClass "NewEnumerator0")
  (|CallParentFunction))