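; End-screen character that shows a winning or losing player with team colors and class-specific montages.
; Winner/loser setup picks Spearman, Bonkerman or Magicman by class-name substring and sets a replicated overlay material from arena and team.
; A server event multicasts animations, where the "Winner" tag selects win or lose montages after fixed or random delays.
; Five-second looping timers are set per class, but their events are empty here.
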(event Custom|SR_PlayAnimations
  (params (PlayerClass :type BP%20Tiki%20Class%20Reference))
  ;[0.15 0.15 0.15 0.5] Animation logic
  (CallFunction|MCPlayanimations PlayerClass))

(event Custom|MC_PlayAnimations
  (params (PlayerClass :type BP%20Tiki%20Class%20Reference))
  ;[0.15 0.15 0.15 0.5] Animation logic
  (Utilities|SwitchonBPTikiClass PlayerClass)
  (switch Utilities|FlowControl|Switch|SwitchonE_CharacterClasses (Variables|Default|GeteCurrentCharacter)
    (:NewEnumerator0
      (Utilities|PlayAnimations true "/Game/Assets/TikiCharacter/Animations/Spearman/AM_LockSpearman.AM_LockSpearman" "/Game/Assets/TikiCharacter/Animations/Shared/AM_LoseAnim.AM_LoseAnim")
      (Utilities|Time|SetTimerbyEvent (delegate Custom|LoopSpearman) 5.0 true)
      (Utilities|PlayAnimations false "/Game/Assets/TikiCharacter/Animations/Spearman/AM_LockSpearman.AM_LockSpearman" "/Game/Assets/TikiCharacter/Animations/Shared/AM_Cry.AM_Cry"))
    (:NewEnumerator1
      (Utilities|PlayAnimations true "/Game/Assets/TikiCharacter/Animations/Bonkerman/AM_BonkermanWin.AM_BonkermanWin" "/Game/Assets/TikiCharacter/Animations/Shared/AM_LoseAnim.AM_LoseAnim")
      (Utilities|Time|SetTimerbyEvent (delegate Custom|LoopBonkerman) 5.0 true)
      (Utilities|PlayAnimations false "/Game/Assets/TikiCharacter/Animations/Bonkerman/AM_LockBonkerman.AM_LockBonkerman" "/Game/Assets/TikiCharacter/Animations/Shared/AM_Cry.AM_Cry"))
    (:NewEnumerator2
      (Utilities|PlayAnimations true "/Game/Assets/TikiCharacter/Animations/Magicman/AM_Magicman_Win.AM_Magicman_Win" "/Game/Assets/TikiCharacter/Animations/Shared/AM_LoseAnim.AM_LoseAnim")
      (Utilities|Time|SetTimerbyEvent (delegate Custom|LoopMagicman) 5.0 true)
      (Utilities|PlayAnimations false "/Game/Assets/TikiCharacter/Animations/Magicman/AM_LockMagicMan.AM_LockMagicMan" "/Game/Assets/TikiCharacter/Animations/Shared/AM_Cry.AM_Cry"))))

(event Custom|LoopMagicman
  ;[0.15 0.15 0.15 0.5] Animation logic
)

(event Custom|LoopSpearman
  ;[0.15 0.15 0.15 0.5] Animation logic
)

(event Custom|LoopBonkerman
  ;[0.15 0.15 0.15 0.5] Animation logic
)

(event EventBeginPlay
  ;[0.15 0.15 0.15 0.5] Animation logic
  (|CallParentFunction))

(fn ConstructionScript
  (|CallParentFunction))

(fn SetTeamColor
  (params (ArenaType :type E_ArenaType%20Enum :default "NewEnumerator0") (WhichTeam :type E_Team%20Enum :default "NewEnumerator0"))
  (switch Utilities|FlowControl|Switch|SwitchonE_ArenaType ArenaType
    (:NewEnumerator0
      (switch Utilities|FlowControl|Switch|SwitchonE_Team WhichTeam
        (:NewEnumerator0
          (Variables|Default|SetmOverlayMaterial "/Game/Assets/TikiCharacter/Materials/MI_RedPlayer.MI_RedPlayer"))
        (:NewEnumerator1
          (Variables|Default|SetmOverlayMaterial "/Game/Assets/TikiCharacter/Materials/MI_BluePlayer.MI_BluePlayer"))))
    (:NewEnumerator1
      (switch Utilities|FlowControl|Switch|SwitchonE_Team WhichTeam
        (:NewEnumerator0
          (Variables|Default|SetmOverlayMaterial "/Game/Assets/TikiCharacter/Materials/MI_PurplePLayer.MI_PurplePLayer"))
        (:NewEnumerator1
          (Variables|Default|SetmOverlayMaterial "/Game/Assets/TikiCharacter/Materials/MI_YellowPlayer.MI_YellowPlayer"))))))

(fn OnRepMOverlayMaterial
  (Rendering|Material|SetOverlayMaterial (Variables|Character|GetMesh) (Variables|Default|GetmOverlayMaterial) :!class /Script/Engine.MeshComponent))

(fn SetLoserTeam
  (params (PlayerClass :type BP%20Tiki%20Class%20Reference) (ArenaType :type E_ArenaType%20Enum :default "NewEnumerator0") (WhichTeam :type E_Team%20Enum :default "NewEnumerator0"))
  (Utilities|SwitchonBPTikiClass PlayerClass)
  (CallFunction|SetTeamColor ArenaType WhichTeam))

(fn SetWinnerTeam
  (params (PlayerClass :type BP%20Tiki%20Class%20Reference) (ArenaType :type E_ArenaType%20Enum :default "NewEnumerator0") (WhichTeam :type E_Team%20Enum :default "NewEnumerator0"))
  (Utilities|SwitchonBPTikiClass PlayerClass)
  (CallFunction|SetTeamColor ArenaType WhichTeam))

(fn OnRepASadAnimation
  (Components|SkeletalMesh|SetAnimInstanceClass (Variables|Character|GetMesh) (Variables|Default|GetaSadAnimation)))