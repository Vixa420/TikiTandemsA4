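; Breakable pillar obstacle whose six totem stairs rise one by one after a random delay at BeginPlay, with sound, dust and camera shake.
; The first Tiki on top claims it, walking slower with a doubled damage multiplier.
; A second Tiki, or another player's projectile while occupied, triggers stun damage and physics collapse of the pillar.
; Projectile hits also fling debris by velocity and later lower the totems in reverse order.
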(event OnComponentBeginOverlap(TopCollision)
  (params (OverlappedComponent :type Primitive%20Component%20Object%20Reference) (OtherActor :type Actor%20Object%20Reference) (OtherComp :type Primitive%20Component%20Object%20Reference) (OtherBodyIndex :type Integer) (bFromSweep :type Boolean) (SweepResult :type Hit%20Result%20Structure%20%28by%20ref%29))
  ;[1 1 1] StandingPlayerOnPillarLogic
  (if (Variables|Default|GetbIsTaken?)
    (bind _asbp_tiki (Utilities|Casting|CastToBP_Tiki OtherActor))
    (Utilities|FlowControl|Delay 0.2)
    (Variables|Default|SetAnotherPlayer _asbp_tiki)
    (CallFunction|BreakPlatform)
    (else
      (bind _asbp_tiki_2 (Utilities|Casting|CastToBP_Tiki OtherActor))
      (bind _output_get (Variables|Default|SetOwningPlayer _asbp_tiki_2))
      (Variables|Default|SetfCharacterWalkSpeed (Variables|/Game/Core/Blueprints/TikiCharacter/Blueprint/BP_Tiki.BP_Tiki_C|GetfDefaultWalkSpeed _output_get))
      (Variables|/Script/Engine.CharacterMovementComponent|SetMaxWalkSpeed (Variables|/Script/Engine.Character|GetCharacterMovement _output_get) 2e+02)
      (Variables|Default|SetbIsTaken? true)
      (Variables|/Game/Core/Blueprints/TikiCharacter/Blueprint/BP_Tiki.BP_Tiki_C|SetfDamageMultiplier _output_get 2.0))))

(event OnComponentEndOverlap(TopCollision)
  (params (OverlappedComponent :type Primitive%20Component%20Object%20Reference) (OtherActor :type Actor%20Object%20Reference) (OtherComp :type Primitive%20Component%20Object%20Reference) (OtherBodyIndex :type Integer))
  ;[1 1 1] LeavingPlayerFromPillarLogic
  (if (== OtherActor (Variables|Default|GetOwningPlayer))
    (Variables|Default|SetbIsTaken? false)
    (Variables|/Script/Engine.CharacterMovementComponent|SetMaxWalkSpeed (Variables|/Script/Engine.Character|GetCharacterMovement (Variables|Default|GetOwningPlayer)) (Variables|Default|GetfCharacterWalkSpeed))))

(event OnComponentBeginOverlap(TowerCollision)
  (params (OverlappedComponent :type Primitive%20Component%20Object%20Reference) (OtherActor :type Actor%20Object%20Reference) (OtherComp :type Primitive%20Component%20Object%20Reference) (OtherBodyIndex :type Integer) (bFromSweep :type Boolean) (SweepResult :type Hit%20Result%20Structure%20%28by%20ref%29))
  (bind _returnvalue (Transformation|GetActorForwardVector OtherActor))
  (bind _returnvalue_2 (Transformation|GetVelocity OtherActor))
  (bind _returnvalue_3 (Math|Vector|VectorLengthXY _returnvalue_2))
  (bind _returnvalue_4 (* _returnvalue "100000.000000,100000.000000,0.000000"))
  (bind _returnvalue_5 (Math|Float|NormalizetoRange _returnvalue_3 4e+02 6e+03))
  ;[1 1 1] IfProjectileHitsPillarLogic
  (if (Actor|ActorHasTag OtherActor "Projectile")
    (if (and (!= (Variables|/Script/Engine.Actor|GetInstigator OtherActor) (Variables|Default|GetOwningPlayer)) (Variables|Default|GetbIsTaken?))
      (CallFunction|BreakPlatform)
      (for _array_element (Variables|Default|GetPillarMeshes)
        (Physics|AddForce _array_element (Math|Vector|MakeVector (* (.x _returnvalue_4) _returnvalue_5) (* (.y _returnvalue_4) _returnvalue_5) 1e+03) "None" true))
      (Camera|PlayWorldCameraShake "/Game/Core/Cinematics/CameraShake/BP_SpearCage_CS.BP_SpearCage_CS_C" "0, 0, 0" 5e+02 1e+03)
      (Niagara|SpawnSystematLocation "/Game/Assets/VFX/Flipbook_VFX/Shared/Particles/Dust/NS_DustHit.NS_DustHit" "0, 0, 0" "0, 0, 0" "5.000000,5.000000,5.000000")
      (Class|BPIEIK|BreakPlatforms(Message) (Game|GetInstigatorController OtherActor))
      (Utilities|FlowControl|Delay 3.0)
      (CallFunction|BringDownStairs))))

(event Custom|BringDownStairs
  (bind _totems (Variables|Default|GetTotems))
  (bind _icounter (Variables|Default|GetiCounter))
  (bind _output (Utilities|Array|Get(acopy) _totems _icounter))
  (bind _returnvalue (Transformation|GetWorldLocation _output))
  (bind _returnvalue_2 (Transformation|GetRelativeTransform _output))
  ;[1 1 1] BringDownTotemStairsLogic
  (Utilities|IsValid _output
    (:Is%20Valid
      (Components|MoveComponentTo _output (Math|Vector|MakeVector (.x (.location _returnvalue_2)) (.y (.location _returnvalue_2)) -6.5e+02) (.rotation _returnvalue_2) false true 0.2 false)
      (Niagara|SpawnSystematLocation "/Game/Assets/VFX/Flipbook_VFX/Shared/Particles/Explosions/NS_Fall.NS_Fall" _returnvalue "0, 0, 0" "8.000000,8.000000,8.000000")
      (Camera|PlayWorldCameraShake "/Game/Core/Cinematics/CameraShake/BP_SpearCage_CS.BP_SpearCage_CS_C" _returnvalue 1e+02 3e+02)
      (if (<= (Variables|Default|GetiCounter) 0)
        (Utilities|FlowControl|DoOnce false
          (:Completed
            (CallFunction|ResetUp)))
        (else
          (Math|Integer|DecrementInt (Variables|Default|GetiCounter)
            (:%20%20
              _))))
      (CallFunction|BringDownStairs))))

(event Custom|BringUpStairs
  (bind _totems (Variables|Default|GetTotems))
  (bind _icounter (Variables|Default|GetiCounter))
  (bind _output (Utilities|Array|Get(acopy) _totems _icounter))
  (bind _returnvalue (Transformation|GetWorldLocation _output))
  (bind _returnvalue_2 (Transformation|GetRelativeTransform _output))
  ;[1 1 1] BringUpTotemStairsLogic
  (Utilities|IsValid _output
    (:Is%20Valid
      (Audio|PlaySoundatLocation "/Game/Assets/SFX/Totems_Rising.Totems_Rising" _returnvalue "0, 0, 0" 1.0 1.0 0.0 0 0 0 0)
      (Components|MoveComponentTo _output (Math|Vector|MakeVector (.x (.location _returnvalue_2)) (.y (.location _returnvalue_2)) 0.0) (.rotation _returnvalue_2) true false 0.2 false)
      (Niagara|SpawnSystematLocation "/Game/Assets/VFX/Flipbook_VFX/Shared/Particles/Explosions/NS_Fall.NS_Fall" _returnvalue "0, 0, 0" "8.000000,8.000000,8.000000")
      (Camera|PlayWorldCameraShake "/Game/Core/Cinematics/CameraShake/BP_SpearCage_CS.BP_SpearCage_CS_C" _returnvalue 5e+02 1e+03)
      (if (>= (Variables|Default|GetiCounter) 5)
        (Utilities|FlowControl|DoOnce false
          (:Completed
            (CallFunction|ResetDown)))
        (else
          (Math|Integer|IncrementInt (Variables|Default|GetiCounter)
            (:%20%20
              _))))
      (CallFunction|BringUpStairs))))

(event Custom|ResetDown
  ;[1 1 1] BringDownTotemStairsLogic
  (Utilities|FlowControl|DoOnce false) ; enters at Reset
)

(event Custom|BreakPlatform
  (bind _pillarmeshes (Variables|Default|GetPillarMeshes))
  ;[1 1 1] BreakingThePillarLogic
  (CallFunction|StunPlayers)
  (Components|DestroyComponent (Variables|Default|GetStairsCollision))
  (for _array_element _pillarmeshes
    (Physics|SetSimulatePhysics _array_element true))
  (Utilities|FlowControl|Delay 7.0)
  (for _array_element_2 _pillarmeshes
    (Components|DestroyComponent _array_element_2)))

(event Custom|StunPlayers
  (bind _self self)
  ;[1 1 1] StunningIf2PlayersOnPillarLogic
  (if (Utilities|AreBothPlayersStandingonthePlatform?)
    (Utilities|FlowControl|Sequence
      (:then_0
        (Game|Damage|ApplyDamage (Variables|Default|GetOwningPlayer) 1.0 0 _self "/Game/Core/Data/DamageTypes/DT_Stun.DT_Stun_C" :!label _label))
      (:then_1
        (Game|Damage|ApplyDamage (Variables|Default|GetAnotherPlayer) 1.0 0 _self "/Game/Core/Data/DamageTypes/DT_Stun.DT_Stun_C")))
    (else
      (goto _label))))

(event Custom|ResetUp
  ;[1 1 1] BringUpTotemStairsLogic
  (Utilities|FlowControl|DoOnce false) ; enters at Reset
)

(event EventBeginPlay
  ;[1 1 1] Event BeginPlay
  (Utilities|FlowControl|Delay (Math|Random|RandomFloatinRange 2e+01 6e+01))
  (CallFunction|BringUpStairs))

(fn ConstructionScript
  (Utilities|SetPillarMeshes)
  (bind _output_get (Utilities|SetTotems))
  (for _array_element _output_get
    (Transformation|SetRelativeLocation _array_element (Math|Vector|MakeVector (.x (Variables|/Script/Engine.SceneComponent|GetRelativeLocation _array_element)) (.y (Variables|/Script/Engine.SceneComponent|GetRelativeLocation _array_element)) -6.9e+02) false false)))