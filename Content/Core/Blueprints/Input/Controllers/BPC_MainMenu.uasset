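; Main menu player controller that creates the custom menu widget in UI-only input mode and handles combat hotkey rebinding.
; Entering remapping mode switches to game-only input, so the next AnyKey press remaps the chosen action in IMCCombat, relabels its widget and restores UI input.
; Custom bindings live in a hotkey map written to the settings save, and a reset event restores attack and jump defaults.
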(event EventBeginPlay
  (bind _self self)
  (Input|SetInputModeUIOnly _self 0 "DoNotLock" false)
  (Variables|Default|SetbShowMouseCursor true)
  (bind _returnvalue (UserInterface|CreateWidget "/Game/Core/Widgets/NewWidgets/W_CustomMainMenu.W_CustomMainMenu_C" _self))
  (bind _output_get (Variables|Default|SetwMainMenu _returnvalue))
  (UserInterface|Viewport|AddtoViewport _output_get 0))

(event Custom|Reset%20Hotkeys
  (bind _imc_combat (Variables|Default|GetIMC%20Combat))
  (bind _imc_combat_2 (Variables|Default|GetIMC%20Combat))
  (bind _imc_combat_3 (Variables|Default|GetIMC%20Combat))
  (bind _imc_combat_4 (Variables|Default|GetIMC%20Combat))
  (bind _default_hotkey_map (Variables|Default|GetDefault%20Hotkey%20Map))
  (Class|InputMappingContext|UnmapAllKeysfromAction _imc_combat_2 "/Game/Core/Blueprints/Input/InputActions/IA_HeavyAttack.IA_HeavyAttack")
  (Class|InputMappingContext|MapKey _imc_combat_2 "/Game/Core/Blueprints/Input/InputActions/IA_HeavyAttack.IA_HeavyAttack" (.Value (Utilities|Map|Find (Variables|Default|GetDefault%20Hotkey%20Map) "/Game/Core/Blueprints/Input/InputActions/IA_HeavyAttack.IA_HeavyAttack")))
  (Class|InputMappingContext|UnmapAllKeysfromAction _imc_combat_3 "/Game/Core/Blueprints/Input/InputActions/IA_BasicAttack.IA_BasicAttack")
  (Class|InputMappingContext|MapKey _imc_combat_3 "/Game/Core/Blueprints/Input/InputActions/IA_BasicAttack.IA_BasicAttack" (.Value (Utilities|Map|Find (Variables|Default|GetDefault%20Hotkey%20Map) "/Game/Core/Blueprints/Input/InputActions/IA_BasicAttack.IA_BasicAttack")))
  (Class|InputMappingContext|UnmapAllKeysfromAction _imc_combat_4 "/Game/Core/Blueprints/Input/InputActions/IA_Jump.IA_Jump")
  (Class|InputMappingContext|MapKey _imc_combat_4 "/Game/Core/Blueprints/Input/InputActions/IA_Jump.IA_Jump" (.Value (Utilities|Map|Find (Variables|Default|GetDefault%20Hotkey%20Map) "/Game/Core/Blueprints/Input/InputActions/IA_Jump.IA_Jump")))
  (Class|InputMappingContext|UnmapAllKeysfromAction _imc_combat "/Game/Core/Blueprints/Input/InputActions/IA_SpecialAttack.IA_SpecialAttack")
  (Class|InputMappingContext|MapKey _imc_combat "/Game/Core/Blueprints/Input/InputActions/IA_SpecialAttack.IA_SpecialAttack" (.Value (Utilities|Map|Find (Variables|Default|GetDefault%20Hotkey%20Map) "/Game/Core/Blueprints/Input/InputActions/IA_SpecialAttack.IA_SpecialAttack")))
  (Variables|Default|SetCustomHotkeyMap _default_hotkey_map)
  (Variables|/Game/Core/Blueprints/SaveGame/BP_SaveGameSettings.BP_SaveGameSettings_C|SetCustomHotkeyMap (.Settings%20Save (CallFunction|GetSettingsSave)) _default_hotkey_map)
  (CallFunction|SaveGameSettings))

(event Custom|EnterRemappingMode
  (params (ActionToRemap :type Input%20Action%20Object%20Reference) (WidgetToRename :type W%20Custom%20Button%20Object%20Reference))
  (bind _self self)
  (Variables|Default|SetWidget%20to%20Rename WidgetToRename)
  (Variables|Default|SetAction%20to%20Remap ActionToRemap)
  (Input|SetInputModeGameOnly _self false)
  (Variables|Default|SetbShowMouseCursor _self false))

(event Input|KeyboardEvents|AnyKey
  (params (Key :type Key%20Structure :default "None"))
  (bind _self self)
  (bind _action_to_remap (Variables|Default|GetAction%20to%20Remap))
  (bind _imc_combat (Variables|Default|GetIMC%20Combat))
  (:Pressed
    (Variables|Default|SetNewHotkey Key)
    (Class|InputMappingContext|UnmapKey _imc_combat _action_to_remap (.Value (Utilities|Map|Find (Variables|Default|GetCustomHotkeyMap) _action_to_remap)))
    (Class|InputMappingContext|MapKey _imc_combat (Variables|Default|GetAction%20to%20Remap) (Variables|Default|GetNewHotkey))
    (Utilities|Map|Remove (Variables|Default|GetCustomHotkeyMap) (Variables|Default|GetAction%20to%20Remap))
    (Utilities|Map|Add (Variables|Default|GetCustomHotkeyMap) (Variables|Default|GetAction%20to%20Remap) (Variables|Default|GetNewHotkey))
    (Input|SetInputModeUIOnly _self 0 "DoNotLock" false)
    (Variables|Default|SetbShowMouseCursor _self true)
    (Variables|/Game/Core/Widgets/NewWidgets/W_CustomButton.W_CustomButton_C|SetButtonText (Variables|Default|GetWidget%20to%20Rename) (Class|KismetInputLibrary|KeyGetDisplayName (Variables|Default|GetNewHotkey) false))
    (Variables|/Game/Core/Blueprints/SaveGame/BP_SaveGameSettings.BP_SaveGameSettings_C|SetCustomHotkeyMap (.Settings%20Save (CallFunction|GetSettingsSave)) (Variables|Default|GetCustomHotkeyMap))
    (CallFunction|SaveGameSettings)))

(fn ConstructionScript)