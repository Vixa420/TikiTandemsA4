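; Player controller for the Training Grounds that runs character selection, explanation screens and the training HUD.
; It spawns the game instance's chosen class at the TrainingStart-tagged transform, possesses it and adds the combat input mapping.
; Enhanced Input is forwarded to the BP_Tiki pawn, with attacks gated by enable flags and Exit toggling character selection.
; Pause and resume events swap widgets and input modes, with camera switches and loading screens around selection.
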(event Custom|HUDHidden
  (Widget|RemovefromParent (Variables|Default|GetwTrainingHUD)))

(event Custom|HUDVisible
  (UserInterface|Viewport|AddtoViewport (Variables|Default|GetwTrainingHUD) 0))

(event Custom|BeginTraining
  (CallFunction|RemoveLoadingScreen)
  (bind _returnvalue (UserInterface|CreateWidget "/Game/Core/Widgets/TrainingGrounds/W_CharacterSelection_Training.W_CharacterSelection_Training_C"))
  (bind _output_get (Variables|Default|SetwCharSelHUD _returnvalue))
  (UserInterface|Viewport|AddtoViewport _output_get 0)
  (CallFunction|CharacterSelectionPause))

(event Custom|ExplanationResume
  (CallFunction|GeneralResume)
  (Widget|RemovefromParent (Variables|Default|GetwExplanation))
  (CallFunction|HUDVisible))

(event Custom|ExplanationPause
  (CallFunction|GeneralPause)
  (UserInterface|Viewport|AddtoViewport (Variables|Default|GetwExplanation) 0)
  (CallFunction|HUDHidden))

(event Custom|CharacterSelectionPause
  (bind _self self)
  (bind _wcharselhud (Variables|Default|GetwCharSelHUD))
  (Input|SetInputModeUIOnly _self (Variables|/Game/Core/Widgets/TrainingGrounds/W_CharacterSelection_Training.W_CharacterSelection_Training_C|GetSpearman _wcharselhud) "DoNotLock" false)
  (Variables|Default|SetbShowMouseCursor _self true)
  (UserInterface|Viewport|AddtoViewport _wcharselhud 0)
  (bind _returnvalue (Actor|GetActorOfClass "/Script/Engine.CameraActor"))
  (Game|Player|SetViewTargetwithBlend _self _returnvalue 0.0 "VTBlend_Linear" 0.0 false)
  (Widget|RemovefromParent (Variables|Default|GetwTrainingHUD)))

(event Custom|CharacterSelectionResume
  (UserInterface|Viewport|AddtoViewport (Variables|Default|GetLoading%20Screen%20Widget) 0)
  (CallFunction|GeneralResume)
  (Widget|RemovefromParent (Variables|Default|GetwCharSelHUD))
  (Game|Player|SetViewTargetwithBlend self (Pawn|GetControlledPawn) 0.0 "VTBlend_Linear" 0.0 false)
  (UserInterface|Viewport|AddtoViewport (Variables|Default|GetwTrainingHUD) 0)
  (Utilities|FlowControl|Delay 0.2)
  (CallFunction|RemoveLoadingScreen))

(event Custom|SpawnAndPlay
  (CallFunction|SpawnCharacter)
  (CallFunction|CharacterSelectionResume)
  (CallFunction|ExplanationPause))

(event Custom|CreateHUDS
  (Utilities|FlowControl|DoOnce false
    (:Completed
      (CallFunction|SetCurrentQuest "1")
      (CallFunction|ExplanationPause))))

(event Custom|LoadingScreen
  ;[1 1 1] Show loading screen
  (bind _loadingscreenwidget (CallFunction|CreateLoadingScreen self))
  (Variables|Default|SetLoading%20Screen%20Widget _loadingscreenwidget))

(event Custom|CreateArenaExplanation
  (bind _returnvalue (UserInterface|CreateWidget "/Game/Core/Widgets/TrainingGrounds/ExplanationWidgets/W_TotemExplanation.W_TotemExplanation_C"))
  (bind _output_get (Variables|Default|SetwTotemExplanation _returnvalue))
  (UserInterface|Viewport|AddtoViewport _output_get 0)
  (CallFunction|HUDHidden)
  (Widget|SetVisibility (Variables|/Game/Core/Widgets/TrainingGrounds/W_TrainingGroundsOverlay.W_TrainingGroundsOverlay_C|GetW_Score_Training (Variables|Default|GetwTrainingHUD)) "Visible"))

(event Custom|RemoveLoadingScreen
  ;[1 1 1] Show loading screen
  (Widget|RemovefromParent (Variables|Default|GetLoading%20Screen%20Widget)))

(event Custom|GeneralResume
  (bind _self self)
  (Input|SetInputModeGameOnly _self false)
  (Variables|Default|SetbShowMouseCursor _self false)
  (Input|EnableInput _self))

(event Custom|GeneralPause
  (bind _self self)
  (Input|SetInputModeUIOnly _self 0 "DoNotLock" false)
  (Variables|Default|SetbShowMouseCursor _self true)
  (Input|DisableInput _self))

(event Input|EnhancedActionEvents|EnhancedInputActionIA_Look
  (params (ActionValue :type Vector%202D%20Structure) (ElapsedSeconds :type Float%20%28double-precision%29) (TriggeredSeconds :type Float%20%28double-precision%29) (InputAction :type Input%20Action%20Object%20Reference :default "/Game/Core/Blueprints/Input/InputActions/IA_Look.IA_Look"))
  ;[1 1 1] Basic input
  (Default|LookInput (Variables|Default|GetBPTikiReference) (.x ActionValue) (.y ActionValue)))

(event Input|EnhancedActionEvents|EnhancedInputActionIA_Move
  (params (ActionValue :type Vector%202D%20Structure) (ElapsedSeconds :type Float%20%28double-precision%29) (TriggeredSeconds :type Float%20%28double-precision%29) (InputAction :type Input%20Action%20Object%20Reference :default "/Game/Core/Blueprints/Input/InputActions/IA_Move.IA_Move"))
  ;[1 1 1] Basic input
  (Default|MoveInput (Variables|Default|GetBPTikiReference) (.x ActionValue) (.y ActionValue)))

(event Input|EnhancedActionEvents|EnhancedInputActionIA_Jump
  (params (ActionValue :type Boolean) (ElapsedSeconds :type Float%20%28double-precision%29) (TriggeredSeconds :type Float%20%28double-precision%29) (InputAction :type Input%20Action%20Object%20Reference :default "/Game/Core/Blueprints/Input/InputActions/IA_Jump.IA_Jump"))
  ;[1 1 1] Basic input
  (:Started
    (Default|JumpInput (Variables|Default|GetBPTikiReference))))

(event Input|EnhancedActionEvents|EnhancedInputActionIA_BasicAttack
  (params (ActionValue :type Boolean) (ElapsedSeconds :type Float%20%28double-precision%29) (TriggeredSeconds :type Float%20%28double-precision%29) (InputAction :type Input%20Action%20Object%20Reference :default "/Game/Core/Blueprints/Input/InputActions/IA_BasicAttack.IA_BasicAttack"))
  (bind _bisbasicenabled (Variables|Default|GetbIsBasicEnabled))
  (bind _bptikireference (Variables|Default|GetBPTikiReference))
  ;[1 1 1] Combat input
  (:Triggered
    (if _bisbasicenabled
      (Class|BPICombat|ICBasicAttackTriggered(Message) _bptikireference ElapsedSeconds)))
  (:Started
    (if _bisbasicenabled
      (Class|BPICombat|ICBasicAttackStarted(Message) _bptikireference)))
  (:Completed
    (if _bisbasicenabled
      (Class|BPICombat|ICBasicAttackCompleted(Message) _bptikireference))))

(event Input|EnhancedActionEvents|EnhancedInputActionIA_SpecialAttack
  (params (ActionValue :type Boolean) (ElapsedSeconds :type Float%20%28double-precision%29) (TriggeredSeconds :type Float%20%28double-precision%29) (InputAction :type Input%20Action%20Object%20Reference :default "/Game/Core/Blueprints/Input/InputActions/IA_SpecialAttack.IA_SpecialAttack"))
  ;[1 1 1] Combat input
  (:Started
    (if (Variables|Default|GetbIsSpecialEnabled)
      (Class|BPICombat|ICSpecialAttackStarted(Message) (Variables|Default|GetBPTikiReference)))))

(event Input|EnhancedActionEvents|EnhancedInputActionIA_HeavyAttack
  (params (ActionValue :type Boolean) (ElapsedSeconds :type Float%20%28double-precision%29) (TriggeredSeconds :type Float%20%28double-precision%29) (InputAction :type Input%20Action%20Object%20Reference :default "/Game/Core/Blueprints/Input/InputActions/IA_HeavyAttack.IA_HeavyAttack"))
  ;[1 1 1] Combat input
  (:Started
    (if (Variables|Default|GetbIsHeavyEnabled)
      (Class|BPICombat|ICHeavyAttackStarted(Message) (Variables|Default|GetBPTikiReference)))))

(event Input|EnhancedActionEvents|EnhancedInputActionIA_Exit
  (params (ActionValue :type Boolean) (ElapsedSeconds :type Float%20%28double-precision%29) (TriggeredSeconds :type Float%20%28double-precision%29) (InputAction :type Input%20Action%20Object%20Reference :default "/Game/Core/Blueprints/Input/InputActions/IA_Exit.IA_Exit"))
  ;[1 1 1] Combat input
  (:Started
    (Utilities|FlowControl|FlipFlop
      (:A
        (CallFunction|CharacterSelectionPause))
      (:B
        (CallFunction|CharacterSelectionResume)))))

(event Input|EnhancedActionEvents|EnhancedInputActionIA_HideExplanation
  (params (ActionValue :type Boolean) (ElapsedSeconds :type Float%20%28double-precision%29) (TriggeredSeconds :type Float%20%28double-precision%29) (InputAction :type Input%20Action%20Object%20Reference :default "/Game/Core/Blueprints/Input/InputActions/IA_HideExplanation.IA_HideExplanation"))
  (:Started
    (Default|ExplanationAnimation (Variables|Default|GetwTrainingHUD))))

(event EventBeginPlay
  ;[1 1 1] Begin play
  (CallFunction|LoadingScreen)
  (bind _returnvalue (UserInterface|CreateWidget "/Game/Core/Widgets/TrainingGrounds/W_TrainingGroundsOverlay.W_TrainingGroundsOverlay_C"))
  (Variables|Default|SetwTrainingHUD _returnvalue)
  (bind _returnvalue_2 (UserInterface|CreateWidget "/Game/Core/Widgets/TrainingGrounds/W_ExplanationWidget.W_ExplanationWidget_C"))
  (Variables|Default|SetwExplanation _returnvalue_2)
  (Utilities|FlowControl|DoOnce false
    (:Completed
      (bind _outactors (Actor|GetAllActorswithTag "TrainingStart"))
      (Variables|Default|SettSpawnPos (Transformation|GetActorTransform (Utilities|Array|Get(acopy) _outactors))))))

(fn ConstructionScript)

(fn SpawnCharacter
  (bind _tspawnpos (Variables|Default|GettSpawnPos))
  (bind _asgi_tiki_tandems (Utilities|Casting|CastToGI_TikiTandems (Game|GetGameInstance)))
  (bind _returnvalue (Game|SpawnActorfromClass (Variables|/Game/Core/Blueprints/GameRules/GI_TikiTandems.GI_TikiTandems_C|GetPlayerClass _asgi_tiki_tandems) (Math|Transform|MakeTransform (.location _tspawnpos) (.rotation _tspawnpos) "1.000000,1.000000,1.000000") "AlwaysSpawn" "MultiplyWithRoot" 0 false false false false 0))
  (Pawn|Possess _returnvalue)
  (CallFunction|AddInputMappingContext self "/Game/Core/Blueprints/Input/InputActionMappings/IMC_Combat.IMC_Combat")
  (bind _asbp_tiki (Utilities|Casting|CastToBP_Tiki (Pawn|GetControlledPawn)))
  (Variables|Default|SetBPTikiReference _asbp_tiki)
  (CallFunction|CreateHUDS))