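; Player controller for the two-player character selection lobby, handling character cycling, lock-in and the handoff to arena choice.
; Server/multicast RPCs sync switches, unlocks and skins, while RepNotifies save the chosen class to the GameInstance, show locked-character feedback and swap input contexts.
; Once both players lock, arena selection opens with input for the host only, identified by player index 0.
; If the host exits, P2 starts a new server.
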(event Custom|CL_SetPlayerClass
  ;[1 1 1] SetPlayerClass in GI logic
  (bind _characterclass (CallFunction|GetPlayerCharacterClass (Variables|Default|GeteSelectedCharacter)))
  (bind _asgi_tiki_tandems (Utilities|Casting|CastToGI_TikiTandems (Game|GetGameInstance)))
  (Variables|/Game/Core/Blueprints/GameRules/GI_TikiTandems.GI_TikiTandems_C|SetPlayerClass _asgi_tiki_tandems _characterclass))

(event Custom|CL_EnableP2
  (bind _characterselectionref (Variables|Default|GetCharacterSelectionRef))
  ;[1 1 1] ShowP2 On joining
  (Rendering|SetActorHiddenInGame (Variables|Default|GetP2ClassName) false)
  (Widget|SetVisibility (Variables|/Game/Core/Widgets/CharacterSelection/W_CharacterSelectionScreen.W_CharacterSelectionScreen_C|GetWaitingP2 _characterselectionref) "Hidden")
  (Widget|SetVisibility (Variables|/Game/Core/Widgets/CharacterSelection/W_CharacterSelectionScreen.W_CharacterSelectionScreen_C|GetW_P2Name _characterselectionref) "Visible"))

(event Custom|MC_LockCharacter
  (params (Target :type BP%20Character%20Selection%20Object%20Reference) (WorldButton :type W%20World%20Button%20Object%20Reference) (Condition :type Boolean))
  ;[1 1 1] Lock character and arena logic
  (if Condition
    (Default|LockCharacter Target WorldButton)
    (Utilities|FlowControl|FlipFlop
      (:A
        (Variables|Default|SetP2Locked? true)
        (Utilities|FlowControl|Delay 0.01)
        (if (Utilities|AreBothPlayersReady?)
          (Default|OpenArenaSelectionMenu (Variables|Default|GetGSCharacterSelectionRef))))
      (:B
        (Variables|Default|SetP2Locked? false)))))

(event Custom|SR_LockCharacter
  (params (Target :type BP%20Character%20Selection%20Object%20Reference) (WorldButton :type W%20World%20Button%20Object%20Reference) (Condition :type Boolean))
  ;[1 1 1] Lock character and arena logic
  (CallFunction|MCLockCharacter Target WorldButton Condition))

(event Custom|CL_SetUnlocks
  ;[1 1 1] CharacterSelection replication logic
  (CallFunction|SetUnlocks)
  (Variables|/Game/Core/Blueprints/Characters/CharacterSelector/BP_CharacterSelection.BP_CharacterSelection_C|SeteCurrentCharacter (Variables|Default|GetPlayerActor) "NewEnumerator0"))

(event Custom|StartGame
  ;[1 1 1] Start the game logic
  (Default|LockArena (Variables|Default|GetCharacterSelectionRef))
  (Default|ArenaChosen (Variables|Default|GetGSCharacterSelectionRef)))

(event Custom|CL_DisableP2
  (bind _characterselectionref (Variables|Default|GetCharacterSelectionRef))
  ;[1 1 1] ShowP2 On joining
  (Rendering|SetActorHiddenInGame (Variables|Default|GetP2ClassName) true)
  (Widget|SetVisibility (Variables|/Game/Core/Widgets/CharacterSelection/W_CharacterSelectionScreen.W_CharacterSelectionScreen_C|GetWaitingP2 _characterselectionref) "Visible")
  (Widget|SetVisibility (Variables|/Game/Core/Widgets/CharacterSelection/W_CharacterSelectionScreen.W_CharacterSelectionScreen_C|GetW_P2Name _characterselectionref) "Hidden"))

(event Custom|LeaveGame
  ;[1 1 1] Server leaving and Client creating new match as Server logic
  (Utilities|Time|ClearandInvalidateTimerbyHandle (stale Input|EnhancedActionEvents|EnhancedInputActionIA_Exit _returnvalue))
  (Game|OpenLevel(byObjectReference) "/Game/maps/L_MainMenu.L_MainMenu"))

(event Custom|StartNewServer
  ;[1 1 1] Server leaving and Client creating new match as Server logic
  (CallFunction|CLLoadingScreen)
  (bind _asgi_tiki_tandems (Utilities|Casting|CastToGI_TikiTandems (Game|GetGameInstance)))
  (Utilities|FlowControl|Delay 1.0)
  (Default|StartNewServer _asgi_tiki_tandems))

(event Custom|SetStencil
  (params (Target :type BP%20Character%20Selection%20Object%20Reference) (CharacterMeshArray :type Array%20of%20Primitive%20Component%20Object%20References) (Stencil :type Integer))
  ;[1 1 1] CharacterSelection replication logic
  (Networking|SwitchHasAuthority
    (:Authority
      (Default|MCSetStencil Target CharacterMeshArray Stencil))
    (:Remote
      (Default|SRSetStencil Target CharacterMeshArray Stencil))))

(event Custom|SR_SetData
  (params (Bonkerman%20Unlocked :type Boolean) (Magicman%20Unlocked :type Boolean) (VoodoomanUnlocked :type Boolean) (BonkermanSkinSet :type Boolean) (MagicmanSkinSet :type Boolean) (SpearmanSkinSet :type Boolean) (VoodooSkinSet :type Boolean) (Target :type BP%20Character%20Selection%20Object%20Reference))
  ;[1 1 1] CharacterSelection replication logic
  (Variables|/Game/Core/Blueprints/Characters/CharacterSelector/BP_CharacterSelection.BP_CharacterSelection_C|SetBonkerman%20Unlocked Target Bonkerman%20Unlocked)
  (Variables|/Game/Core/Blueprints/Characters/CharacterSelector/BP_CharacterSelection.BP_CharacterSelection_C|SetMagicman%20Unlocked Target Magicman%20Unlocked)
  (Variables|/Game/Core/Blueprints/Characters/CharacterSelector/BP_CharacterSelection.BP_CharacterSelection_C|SetVoodoomanUnlocked Target VoodoomanUnlocked)
  (Variables|/Game/Core/Blueprints/Characters/CharacterSelector/BP_CharacterSelection.BP_CharacterSelection_C|SetBonkermanSkinSet Target BonkermanSkinSet)
  (Variables|/Game/Core/Blueprints/Characters/CharacterSelector/BP_CharacterSelection.BP_CharacterSelection_C|SetMagicmanSkinSet Target MagicmanSkinSet)
  (Variables|/Game/Core/Blueprints/Characters/CharacterSelector/BP_CharacterSelection.BP_CharacterSelection_C|SetSpearmanSkinSet Target SpearmanSkinSet)
  (Variables|/Game/Core/Blueprints/Characters/CharacterSelector/BP_CharacterSelection.BP_CharacterSelection_C|SetVoodoomanSkinSet Target VoodooSkinSet))

(event Custom|MC_SetData
  (params (Bonkerman%20Unlocked :type Boolean) (Magicman%20Unlocked :type Boolean) (VoodoomanUnlocked :type Boolean) (BonkermanSkinSet :type Boolean) (MagicmanSkinSet :type Boolean) (SpearmanSkinSet :type Boolean) (VoodooSkinSet :type Boolean) (Target :type BP%20Character%20Selection%20Object%20Reference))
  ;[1 1 1] CharacterSelection replication logic
  (CallFunction|SRSetData Bonkerman%20Unlocked Magicman%20Unlocked VoodoomanUnlocked BonkermanSkinSet MagicmanSkinSet SpearmanSkinSet VoodooSkinSet Target))

(event Custom|CL_AddInputToOwningPlayer
  ;[1 1 1] Add input
  (CallFunction|AddInputMappingContext self "/Game/Core/Blueprints/Input/InputActionMappings/IMC_CharacterSelection.IMC_CharacterSelection"))

(event Custom|CL_GetPlayerRank
  (bind _asgi_tiki_tandems (Utilities|Casting|CastToGI_TikiTandems (Game|GetGameInstance)))
  (Variables|Default|SetPlayerLevel (.Value (Utilities|Map|Find (Variables|/Game/Core/Blueprints/SaveGame/BP_SaveGameSettings.BP_SaveGameSettings_C|GetPlayerStats (Variables|/Game/Core/Blueprints/GameRules/GI_TikiTandems.GI_TikiTandems_C|GetSettings%20Save _asgi_tiki_tandems)) "LEVEL"))))

(event Custom|CL_LoadingScreen
  ;[1 1 1] Show loading screen
  (bind _loadingscreenwidget (CallFunction|CreateLoadingScreen self))
  (bind _output_get (Variables|Default|SetwLoadingScreen _loadingscreenwidget))
  (Utilities|FlowControl|Delay 1.0)
  (Widget|RemovefromParent _output_get))

(event Custom|CL_LobbySetup
  (params (PlayerIndex :type Integer))
  ;[1 1 1] Lobby setup logic
  (Input|SetInputModeGameOnly self true)
  (CallFunction|CLCreateWidgets)
  (CallFunction|SetSelectedPlayer PlayerIndex))

(event Custom|MC_SwitchCharacter
  (params (NextPrev :type Boolean) (WhichPlayer? :type BP%20Character%20Selection%20Object%20Reference))
  ;[1 1 1] Character and map switching logic
  (CallFunction|SwitchCharacter NextPrev WhichPlayer?))

(event Custom|SR_SwitchCharacter
  (params (NextPrev :type Boolean) (WhichPlayer? :type BP%20Character%20Selection%20Object%20Reference))
  ;[1 1 1] Character and map switching logic
  (CallFunction|MCSwitchCharacter NextPrev WhichPlayer?))

(event Custom|ChooseArena
  (bind _returnvalue (Utilities|IsServer?))
  (bind _self self)
  ;[1 1 1] Set arena widget logic
  (Default|ChooseArena (Variables|Default|GetCharacterSelectionRef) _returnvalue)
  (if _returnvalue
    (CallFunction|AddInputMappingContext _self "/Game/Core/Blueprints/Input/InputActionMappings/IMC_CharacterSelection.IMC_CharacterSelection" 1)
    (CallFunction|RemoveInputMappingContext _self "/Game/Core/Blueprints/Input/InputActionMappings/IMC_Lock.IMC_Lock")
    (bind _asgm_character_selection (Utilities|Casting|CastToGM_CharacterSelection (Game|GetGameMode)))
    (Default|MCSetArenaWidget _asgm_character_selection)
    (else
      (CallFunction|RemoveAllInputMappingContexts _self)
      (CallFunction|SRSetArenaWidget))))

(event Custom|CL_CreateWidgets
  ;[1 1 1] Create widgets logic
  (bind _returnvalue (UserInterface|CreateWidget "/Game/Core/Widgets/CharacterSelection/W_CharacterSelectionScreen.W_CharacterSelectionScreen_C" self))
  (bind _output_get (Variables|Default|SetCharacterSelectionRef _returnvalue))
  (UserInterface|Viewport|AddtoViewport _output_get 0)
  (if (not (Utilities|IsServer?))
    (Variables|/Script/UMG.Widget|SetVisibility (Variables|/Game/Core/Widgets/CharacterSelection/W_CharacterSelectionScreen.W_CharacterSelectionScreen_C|GetWaitingP2 (Variables|Default|GetCharacterSelectionRef)) "Hidden")))

(event Custom|SR_SetArenaWidget
  ;[1 1 1] Set arena widget logic
  (bind _asgm_character_selection (Utilities|Casting|CastToGM_CharacterSelection (Game|GetGameMode)))
  (Default|MCSetArenaWidget _asgm_character_selection))

(event Input|EnhancedActionEvents|EnhancedInputActionIA_NextSelection
  (params (ActionValue :type Boolean) (ElapsedSeconds :type Float%20%28double-precision%29) (TriggeredSeconds :type Float%20%28double-precision%29) (InputAction :type Input%20Action%20Object%20Reference :default "/Game/Core/Blueprints/Input/InputActions/IA_NextSelection.IA_NextSelection"))
  (bind _playeractor (Variables|Default|GetPlayerActor))
  ;[1 1 1] Character and map switching logic
  (:Started
    (Variables|Default|SetbNextPrevious true)
    (if (Utilities|AreBothPlayersReady?)
      (Default|MCSetArena (Variables|Default|GetGSCharacterSelectionRef))
      (elif (Utilities|IsServer?)
        (CallFunction|SwitchCharacter (Variables|Default|GetbNextPrevious) _playeractor)
        (else
          (CallFunction|SRSwitchCharacter (Variables|Default|GetbNextPrevious) _playeractor))))))

(event Input|EnhancedActionEvents|EnhancedInputActionIA_PreviousSelection
  (params (ActionValue :type Boolean) (ElapsedSeconds :type Float%20%28double-precision%29) (TriggeredSeconds :type Float%20%28double-precision%29) (InputAction :type Input%20Action%20Object%20Reference :default "/Game/Core/Blueprints/Input/InputActions/IA_PreviousSelection.IA_PreviousSelection"))
  (bind _playeractor (Variables|Default|GetPlayerActor))
  ;[1 1 1] Character and map switching logic
  (:Started
    (Variables|Default|SetbNextPrevious false)
    (if (Utilities|AreBothPlayersReady?)
      (Default|MCSetArena (Variables|Default|GetGSCharacterSelectionRef))
      (elif (Utilities|IsServer?)
        (CallFunction|SwitchCharacter (Variables|Default|GetbNextPrevious) _playeractor)
        (else
          (CallFunction|SRSwitchCharacter (Variables|Default|GetbNextPrevious) _playeractor))))))

(event Input|EnhancedActionEvents|EnhancedInputActionIA_Next
  (params (ActionValue :type Boolean) (ElapsedSeconds :type Float%20%28double-precision%29) (TriggeredSeconds :type Float%20%28double-precision%29) (InputAction :type Input%20Action%20Object%20Reference :default "/Game/Core/Blueprints/Input/InputActions/IA_Next.IA_Next"))
  (bind _playeractor (Variables|Default|GetPlayerActor))
  (bind _playerclassname (Variables|Default|GetPlayerClassName))
  (bind _bcanlock_ (Variables|Default|GetbCanLock?))
  ;[1 1 1] Lock character and arena logic
  (:Started
    (if (Utilities|AreBothPlayersReady?)
      (Utilities|FlowControl|Delay 0.2)
      (if ActionValue
        (Default|OpenArenaLogic (Variables|Default|GetGSCharacterSelectionRef)))
      (elif (Utilities|IsServer?)
        (if _bcanlock_
          (Default|LockCharacter _playeractor _playerclassname)
          (Utilities|FlowControl|FlipFlop
            (:A
              (Variables|Default|SetP1Locked? true)
              (Utilities|FlowControl|Delay 0.01)
              (if (Utilities|AreBothPlayersReady?)
                (Default|OpenArenaSelectionMenu (Variables|Default|GetGSCharacterSelectionRef))))
            (:B
              (Variables|Default|SetP1Locked? false))))
        (else
          (CallFunction|SRLockCharacter _playeractor _playerclassname _bcanlock_))))))

(event Input|EnhancedActionEvents|EnhancedInputActionIA_Exit
  (params (ActionValue :type Boolean) (ElapsedSeconds :type Float%20%28double-precision%29) (TriggeredSeconds :type Float%20%28double-precision%29) (InputAction :type Input%20Action%20Object%20Reference :default "/Game/Core/Blueprints/Input/InputActions/IA_Exit.IA_Exit"))
  (bind _self self)
  ;[1 1 1] Server leaving and Client creating new match as Server logic
  (:Started
    (Input|DisableInput _self _self)
    (CallFunction|CLLoadingScreen)
    (if (and (Utilities|IsServer?) (Variables|Default|GetbP2))
      (bind _returnvalue (Utilities|Time|SetTimerbyEvent (delegate Custom|LeaveGame) 1.0))
      (bind _asgm_character_selection (Utilities|Casting|CastToGM_CharacterSelection (Game|GetGameMode)))
      (bind _asbpc_character_selection (Utilities|Casting|CastToBPC_CharacterSelection (Utilities|Array|Get(acopy) (Variables|/Game/Core/Blueprints/GameRules/GameModes/GM_CharacterSelection.GM_CharacterSelection_C|GetPlayerControllers _asgm_character_selection) 1)))
      (CallFunction|StartNewServer _asbpc_character_selection)
      (else
        (Game|OpenLevel(byObjectReference) "/Game/maps/L_MainMenu.L_MainMenu")))))

(event EventBeginPlay
  ;[1 1 1] Event BeginPlay
  (Utilities|FlowControl|Sequence
    (:then_0
      (bind _asgs_character_selection (Utilities|Casting|CastToGS_CharacterSelection (Game|GetGameState)))
      (Variables|Default|SetGSCharacterSelectionRef _asgs_character_selection))
    (:then_1
      (CallFunction|CLLoadingScreen)
      (CallFunction|InitializeSelectorData))))

(fn ConstructionScript)

(fn InitializeSelectorData
  (Utilities|FlowControl|Sequence
    (:then_0
      (bind _outactors (Actor|GetAllActorsOfClass "/Game/Core/Blueprints/TikiCharacter/Blueprint/BP_Tiki.BP_Tiki_C"))
      (for (_array_element _array_index) _outactors
        (switch int _array_index
          (:0
            (Variables|Default|SetP1Actor _array_element))
          (:1
            (Variables|Default|SetP2Actor _array_element)))))
    (:then_1
      (bind _outactors_2 (Actor|GetAllActorsOfClass "/Game/Core/Widgets/MainMenu/W_WorldButton.W_WorldButton_C"))
      (for (_array_element_2 _array_index_2) _outactors_2
        (switch int _array_index_2
          (:0
            (Variables|Default|SetP1ClassName _array_element_2))
          (:1
            (Variables|Default|SetP2ClassName _array_element_2)))))
    (:then_2
      (CallFunction|CLGetPlayerRank))))

(fn SwitchCharacter
  (params (NextPrev :type Boolean) (WhichPlayer? :type BP%20Character%20Selection%20Object%20Reference))
  (if NextPrev
    (bind _selectedcharacter (CallFunction|NextCharacter WhichPlayer?))
    (Variables|Default|SeteSelectedCharacter _selectedcharacter)
    (else
      (bind _selectedcharacter_2 (CallFunction|PreviousCharacter WhichPlayer?))
      (Variables|Default|SeteSelectedCharacter _selectedcharacter_2))))

(fn NextCharacter
  (params (Swticher :type BP%20Character%20Selection%20Object%20Reference))
  (Default|FlipAnimation Swticher true)
  (switch Utilities|FlowControl|Switch|SwitchonE_CharacterClasses (Variables|/Game/Core/Blueprints/Characters/CharacterSelector/BP_CharacterSelection.BP_CharacterSelection_C|GeteCurrentCharacter Swticher)
    (:NewEnumerator0
      (bind _output_get (Variables|/Game/Core/Blueprints/Characters/CharacterSelector/BP_CharacterSelection.BP_CharacterSelection_C|SeteCurrentCharacter Swticher "NewEnumerator1"))
      (return _output_get))
    (:NewEnumerator1
      (bind _output_get_2 (Variables|/Game/Core/Blueprints/Characters/CharacterSelector/BP_CharacterSelection.BP_CharacterSelection_C|SeteCurrentCharacter Swticher "NewEnumerator2"))
      (return _output_get_2))
    (:NewEnumerator2
      (bind _output_get_3 (Variables|/Game/Core/Blueprints/Characters/CharacterSelector/BP_CharacterSelection.BP_CharacterSelection_C|SeteCurrentCharacter Swticher "NewEnumerator4"))
      (return _output_get_3))
    (:NewEnumerator4
      (bind _output_get_4 (Variables|/Game/Core/Blueprints/Characters/CharacterSelector/BP_CharacterSelection.BP_CharacterSelection_C|SeteCurrentCharacter Swticher "NewEnumerator0"))
      (return _output_get_4))))

(fn PreviousCharacter
  (params (Switcher :type BP%20Character%20Selection%20Object%20Reference))
  (Default|FlipAnimation Switcher false)
  (switch Utilities|FlowControl|Switch|SwitchonE_CharacterClasses (Variables|/Game/Core/Blueprints/Characters/CharacterSelector/BP_CharacterSelection.BP_CharacterSelection_C|GeteCurrentCharacter Switcher)
    (:NewEnumerator0
      (bind _output_get (Variables|/Game/Core/Blueprints/Characters/CharacterSelector/BP_CharacterSelection.BP_CharacterSelection_C|SeteCurrentCharacter Switcher "NewEnumerator4"))
      (return _output_get))
    (:NewEnumerator1
      (bind _output_get_2 (Variables|/Game/Core/Blueprints/Characters/CharacterSelector/BP_CharacterSelection.BP_CharacterSelection_C|SeteCurrentCharacter Switcher "NewEnumerator0"))
      (return _output_get_2))
    (:NewEnumerator2
      (bind _output_get_3 (Variables|/Game/Core/Blueprints/Characters/CharacterSelector/BP_CharacterSelection.BP_CharacterSelection_C|SeteCurrentCharacter Switcher "NewEnumerator1"))
      (return _output_get_3))
    (:NewEnumerator4
      (bind _output_get_4 (Variables|/Game/Core/Blueprints/Characters/CharacterSelector/BP_CharacterSelection.BP_CharacterSelection_C|SeteCurrentCharacter Switcher "NewEnumerator2"))
      (return _output_get_4))))

(fn GetPlayerCharacterClass
  (params (CharacterSelection :type E_CharacterClasses%20Enum :default "NewEnumerator0"))
  (switch Utilities|FlowControl|Switch|SwitchonE_CharacterClasses CharacterSelection
    (:NewEnumerator0
      (return "/Game/Core/Blueprints/Characters/Spearman/BP_Spearman.BP_Spearman_C"))
    (:NewEnumerator1
      (return "/Game/Core/Blueprints/Characters/Bonkerman/BP_Bonkerman.BP_Bonkerman_C"))
    (:NewEnumerator2
      (return "/Game/Core/Blueprints/Characters/Magicman/BP_Magicman.BP_Magicman_C"))
    (:NewEnumerator4
      (return "/Game/Core/Blueprints/Characters/Voodooman/BP_Voodooman.BP_Voodooman_C"))))

(fn OnRepP1Locked?
  (bind _self self)
  (if (Variables|Default|GetP1Locked?)
    (CallFunction|RemoveInputMappingContext _self "/Game/Core/Blueprints/Input/InputActionMappings/IMC_CharacterSelection.IMC_CharacterSelection")
    (CallFunction|AddInputMappingContext _self "/Game/Core/Blueprints/Input/InputActionMappings/IMC_Lock.IMC_Lock" 1)
    (else
      (CallFunction|RemoveInputMappingContext _self "/Game/Core/Blueprints/Input/InputActionMappings/IMC_Lock.IMC_Lock")
      (CallFunction|AddInputMappingContext _self "/Game/Core/Blueprints/Input/InputActionMappings/IMC_CharacterSelection.IMC_CharacterSelection" 1))))

(fn OnRepP2Locked?
  (bind _self self)
  (bind _p2classname (Variables|Default|GetP2ClassName))
  (if (Variables|Default|GetP2Locked?)
    (CallFunction|RemoveInputMappingContext _self "/Game/Core/Blueprints/Input/InputActionMappings/IMC_CharacterSelection.IMC_CharacterSelection")
    (CallFunction|AddInputMappingContext _self "/Game/Core/Blueprints/Input/InputActionMappings/IMC_Lock.IMC_Lock" 1)
    (Default|UpdateTextColor _p2classname)
    (else
      (CallFunction|RemoveInputMappingContext _self "/Game/Core/Blueprints/Input/InputActionMappings/IMC_Lock.IMC_Lock")
      (CallFunction|AddInputMappingContext _self "/Game/Core/Blueprints/Input/InputActionMappings/IMC_CharacterSelection.IMC_CharacterSelection" 1)
      (Default|UpdateTextColor _p2classname "(R=1.000000,G=1.000000,B=1.000000,A=1.000000)"))))

(fn OnRepESelectedCharacter
  (bind _returnvalue (Game|GetGameInstance))
  (bind _characterselectionref (Variables|Default|GetCharacterSelectionRef))
  (bind _playeractor (Variables|Default|GetPlayerActor))
  (bind _characterselectionref_2 (Variables|Default|GetCharacterSelectionRef))
  (bind _eselectedcharacter (Variables|Default|GeteSelectedCharacter))
  (bind _asgi_tiki_tandems (Utilities|Casting|CastToGI_TikiTandems _returnvalue))
  (CallFunction|CLSetPlayerClass)
  (switch Utilities|FlowControl|Switch|SwitchonE_CharacterClasses (Variables|Default|GeteSelectedCharacter)
    (:NewEnumerator0
      (bind _output_get (Variables|Default|SetbCanLock? true))
      (Utilities|SetStencilMacro _output_get _playeractor (Variables|/Game/Core/Blueprints/Characters/CharacterSelector/BP_CharacterSelection.BP_CharacterSelection_C|GetSpearmanMesh _playeractor)))
    (:NewEnumerator1
      (bind _output_get_2 (Variables|Default|SetbCanLock? (Variables|/Game/Core/Blueprints/GameRules/GI_TikiTandems.GI_TikiTandems_C|GetbBonkermanUnlocked _asgi_tiki_tandems)))
      (Utilities|SetStencilMacro _output_get_2 _playeractor (Variables|/Game/Core/Blueprints/Characters/CharacterSelector/BP_CharacterSelection.BP_CharacterSelection_C|GetBonkermanMesh _playeractor)))
    (:NewEnumerator2
      (bind _output_get_3 (Variables|Default|SetbCanLock? (Variables|/Game/Core/Blueprints/GameRules/GI_TikiTandems.GI_TikiTandems_C|GetbMagicmanUnlocked _asgi_tiki_tandems)))
      (Utilities|SetStencilMacro _output_get_3 _playeractor (Variables|/Game/Core/Blueprints/Characters/CharacterSelector/BP_CharacterSelection.BP_CharacterSelection_C|GetMagicmanMesh _playeractor)))
    (:NewEnumerator4
      (bind _output_get_4 (Variables|Default|SetbCanLock? (Variables|/Game/Core/Blueprints/GameRules/GI_TikiTandems.GI_TikiTandems_C|GetbVoodoomanUnlocked _asgi_tiki_tandems)))
      (Utilities|SetStencilMacro _output_get_4 _playeractor (Variables|/Game/Core/Blueprints/Characters/CharacterSelector/BP_CharacterSelection.BP_CharacterSelection_C|GetVoodoomanMesh _playeractor))))
  (if (Utilities|IsServer?)
    (Utilities|Lock _eselectedcharacter (Variables|/Game/Core/Widgets/CharacterSelection/W_CharacterSelectionScreen.W_CharacterSelectionScreen_C|GetLockedP1Text _characterselectionref_2) (Variables|/Game/Core/Widgets/CharacterSelection/W_CharacterSelectionScreen.W_CharacterSelectionScreen_C|GetLockedCharacterP1 _characterselectionref_2) (Variables|Default|GetbCanLock?))
    (else
      (Utilities|Lock _eselectedcharacter (Variables|/Game/Core/Widgets/CharacterSelection/W_CharacterSelectionScreen.W_CharacterSelectionScreen_C|GetLockedP2Text _characterselectionref) (Variables|/Game/Core/Widgets/CharacterSelection/W_CharacterSelectionScreen.W_CharacterSelectionScreen_C|GetLockedCharacterP2 _characterselectionref) (Variables|Default|GetbCanLock?)))))

(fn SetSelectedPlayer
  (params (PlayerIndex :type Integer))
  (bind _output_get (Variables|Default|SetiPlayerIndex PlayerIndex))
  (switch int _output_get
    (:0
      (Variables|Default|SetPlayerActor (.AsBP%20Character%20Selection (Utilities|Casting|CastToBP_CharacterSelection (Variables|Default|GetP1Actor))))
      (Variables|Default|SetPlayerClassName (Variables|Default|GetP1ClassName)))
    (:1
      (Variables|Default|SetPlayerActor (.AsBP%20Character%20Selection (Utilities|Casting|CastToBP_CharacterSelection (Variables|Default|GetP2Actor))))
      (Variables|Default|SetPlayerClassName (Variables|Default|GetP2ClassName)))))

(fn SetUnlocks
  (bind _playeractor (Variables|Default|GetPlayerActor))
  (bind _asgi_tiki_tandems (Utilities|Casting|CastToGI_TikiTandems (Game|GetGameInstance)))
  (bind _output_get (Variables|/Game/Core/Blueprints/Characters/CharacterSelector/BP_CharacterSelection.BP_CharacterSelection_C|SetBonkerman%20Unlocked _playeractor (Variables|/Game/Core/Blueprints/GameRules/GI_TikiTandems.GI_TikiTandems_C|GetbBonkermanUnlocked _asgi_tiki_tandems)))
  (bind _output_get_2 (Variables|/Game/Core/Blueprints/Characters/CharacterSelector/BP_CharacterSelection.BP_CharacterSelection_C|SetMagicman%20Unlocked _playeractor (Variables|/Game/Core/Blueprints/GameRules/GI_TikiTandems.GI_TikiTandems_C|GetbMagicmanUnlocked _asgi_tiki_tandems)))
  (bind _output_get_3 (Variables|/Game/Core/Blueprints/Characters/CharacterSelector/BP_CharacterSelection.BP_CharacterSelection_C|SetVoodoomanUnlocked _playeractor (Variables|/Game/Core/Blueprints/GameRules/GI_TikiTandems.GI_TikiTandems_C|GetbVoodoomanUnlocked _asgi_tiki_tandems)))
  (bind _output_get_4 (Variables|/Game/Core/Blueprints/Characters/CharacterSelector/BP_CharacterSelection.BP_CharacterSelection_C|SetBonkermanSkinSet _playeractor (.Value (Utilities|Map|Find (Variables|/Game/Core/Blueprints/GameRules/GI_TikiTandems.GI_TikiTandems_C|GetSelectedSkins _asgi_tiki_tandems) "NewEnumerator1"))))
  (bind _output_get_5 (Variables|/Game/Core/Blueprints/Characters/CharacterSelector/BP_CharacterSelection.BP_CharacterSelection_C|SetSpearmanSkinSet _playeractor (.Value (Utilities|Map|Find (Variables|/Game/Core/Blueprints/GameRules/GI_TikiTandems.GI_TikiTandems_C|GetSelectedSkins _asgi_tiki_tandems) "NewEnumerator2"))))
  (bind _output_get_6 (Variables|/Game/Core/Blueprints/Characters/CharacterSelector/BP_CharacterSelection.BP_CharacterSelection_C|SetMagicmanSkinSet _playeractor (.Value (Utilities|Map|Find (Variables|/Game/Core/Blueprints/GameRules/GI_TikiTandems.GI_TikiTandems_C|GetSelectedSkins _asgi_tiki_tandems) "NewEnumerator3"))))
  (bind _output_get_7 (Variables|/Game/Core/Blueprints/Characters/CharacterSelector/BP_CharacterSelection.BP_CharacterSelection_C|SetVoodoomanSkinSet _playeractor (.Value (Utilities|Map|Find (Variables|/Game/Core/Blueprints/GameRules/GI_TikiTandems.GI_TikiTandems_C|GetSelectedSkins _asgi_tiki_tandems) "NewEnumerator4"))))
  (if (Utilities|IsServer?)
    (CallFunction|MCSetData _output_get _output_get_2 _output_get_3 _output_get_4 _output_get_6 _output_get_5 _output_get_7 _playeractor)
    (else
      (CallFunction|SRSetData _output_get _output_get_2 _output_get_3 _output_get_4 _output_get_6 _output_get_5 _output_get_7 _playeractor))))