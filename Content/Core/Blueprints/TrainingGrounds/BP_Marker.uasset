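; BP_Marker is a training grounds trigger that advances the quest line when a BP_Tiki overlaps its collision.
; Respawn markers also save their transform as the controller's spawn point and update quests only once; non-reusable markers destroy themselves.
; It progresses its quest or sets it as current, based on a quest struct comparison.
; Hardcoded quest IDs unlock basic, heavy or special attacks on BPC_TrainingGrounds.
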(event OnComponentBeginOverlap(Collision)
  (params (OverlappedComponent :type Primitive%20Component%20Object%20Reference) (OtherActor :type Actor%20Object%20Reference) (OtherComp :type Primitive%20Component%20Object%20Reference) (OtherBodyIndex :type Integer) (bFromSweep :type Boolean) (SweepResult :type Hit%20Result%20Structure%20%28by%20ref%29))
  (bind _nquestid (Variables|Default|GetnQuestID))
  (Utilities|Casting|CastToBP_Tiki OtherActor)
  (Utilities|FlowControl|Sequence
    (:then_0
      (if (Variables|Default|GetbIsRespawn?)
        (bind _asbpc_training_grounds (Utilities|Casting|CastToBPC_TrainingGrounds (Game|GetPlayerController 0)))
        (Variables|/Game/Core/Blueprints/Input/Controllers/BPC_TrainingGrounds.BPC_TrainingGrounds_C|SettSpawnPos _asbpc_training_grounds (Transformation|GetWorldTransform (Variables|Default|GetCollision)))
        (Utilities|FlowControl|DoOnce false
          (:Completed
            _)))
      (if (Variables|Default|GetbIsReusable?)
        _
        (else
          (Actor|DestroyActor)))
      (if (CallFunction|Equal(stQuest) (CallFunction|GetQuest _nquestid) (CallFunction|GetAnyQuestbyID _nquestid))
        (CallFunction|ProgressQuest _nquestid)
        (else
          (CallFunction|SetCurrentQuest _nquestid))))
    (:then_1
      (CallFunction|SetAttacksEnabled))))

(fn ConstructionScript)

(fn SetAttacksEnabled
  (bind _asbpc_training_grounds (Utilities|Casting|CastToBPC_TrainingGrounds (Game|GetPlayerController 0)))
  (if (== (Variables|Default|GetnQuestID) "5")
    (Variables|/Game/Core/Blueprints/Input/Controllers/BPC_TrainingGrounds.BPC_TrainingGrounds_C|SetbIsBasicEnabled _asbpc_training_grounds true)
    (elif (== (Variables|Default|GetnQuestID) "6")
      (Variables|/Game/Core/Blueprints/Input/Controllers/BPC_TrainingGrounds.BPC_TrainingGrounds_C|SetbIsHeavyEnabled _asbpc_training_grounds true)
      (elif (== (Variables|Default|GetnQuestID) "8")
        (Variables|/Game/Core/Blueprints/Input/Controllers/BPC_TrainingGrounds.BPC_TrainingGrounds_C|SetbIsSpecialEnabled _asbpc_training_grounds true)))))