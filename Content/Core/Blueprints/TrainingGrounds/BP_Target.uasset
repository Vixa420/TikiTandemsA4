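; BP_Target is a training-grounds target that reacts to hits during basic attack training.
; HitTarget flags it as hit, plays a Pullback timeline that rotates its roll, and spawns a dust effect.
; It also scans all BP_Target actors, breaking at the first unhit one.
; A constant-true branch follows that loop and calls FinishedBasicAttackTraining, so the call does not depend on the scan result.
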(event Custom|HitTargetAnimation
  (bind _returnvalue (Transformation|GetActorRotation))
  (Variables|Default|SetbIsHit? true)
  (bind _rotation (Timeline|Pullback Play)
    (:Update
      (Transformation|SetActorRotation (Math|Rotator|MakeRotator _rotation (.pitch _returnvalue) (.yaw _returnvalue))))))

(event Custom|CheckTargets
  (bind _outactors (Actor|GetAllActorsOfClass "BP_Target_C"))
  (bind _array_element (Utilities|Array|ForEachLoopwithBreak _outactors :!label _label)
    (:LoopBody
      (if (not (Variables|BP_Target_C|GetbIsHit? _array_element))
        (goto _label Break)))
    (:Completed
      (if true
        (Default|CallFinishedBasicAttackTraining)))))

(event Custom|HitTarget
  (CallFunction|HitTargetAnimation)
  (CallFunction|CheckTargets)
  (Niagara|SpawnSystematLocation "/Game/Assets/VFX/Flipbook_VFX/Shared/Particles/Dust/NS_SmallDustHit.NS_SmallDustHit" (Transformation|GetWorldLocation (Variables|Default|GetOrientation)))
  (Utilities|FlowControl|DoOnce false))

(fn ConstructionScript)