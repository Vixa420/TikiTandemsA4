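; GM_ArenaTest is an arena test game mode that provides functions for spawning and possessing players at team start positions.
; SpawnAndPossessPlayer destroys the controller's current pawn, spawns the given class and has the controller possess it.
; FindPlayerStartPosition supplies the spawn transform from the first PlayerStart matching the team tag, with no check for a missing match.
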(fn ConstructionScript)

(fn SpawnandPossessPlayer
  (params (PlayerController :type Controller%20Object%20Reference) (Class :type BP%20Tiki%20Class%20Reference) (TeamTag :type Name))
  (bind _returnvalue (Pawn|GetControlledPawn PlayerController))
  (Utilities|IsValid _returnvalue
    (:Is%20Valid
      (Actor|DestroyActor _returnvalue))
    (:Is%20Not%20Valid
      _))
  (bind _returnvalue_2 (Game|SpawnActorfromClass Class (CallFunction|FindPlayerStartPosition TeamTag) "Undefined" "MultiplyWithRoot" 0 0))
  (Pawn|Possess PlayerController _returnvalue_2))

(fn FindPlayerStartPosition
  (params (Tag :type Name))
  (bind _outactors (Actor|GetAllActorsOfClasswithTag "/Script/Engine.PlayerStart" Tag))
  (return (Transformation|GetActorTransform (Utilities|Array|Get(acopy) _outactors))))